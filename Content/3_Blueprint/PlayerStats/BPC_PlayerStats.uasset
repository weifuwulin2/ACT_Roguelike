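; Player stats component that tracks health, overload, Straight (a stagger meter), attack speed, critical chance and shield, initialised from PlayerStats on BeginPlay.
; A shared clamp helper drives most changes, and health, overload and Straight update PlayerHUD bars.
; Zero health triggers a death montage and UI; depleted Straight plays a hit reaction and refills.
; Attack speed and crit functions return values without storing them; shield change logic is unconnected.
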(event Custom|PlayerDead
  ;[1 1 1] 玩家死亡
  (Animation|Montage|PlayMontage (Variables|/Script/Engine.Character|GetMesh (Game|GetPlayerCharacter 0)) "/Game/1_Animations/Character/Hit_React/PlayerDie_Montage.PlayerDie_Montage"
    (:then
      (Input|SetInputModeUIOnly (Game|GetPlayerController 0) 0 "DoNotLock" false)
      (bind _returnvalue (UserInterface|CreateWidget "/Game/3_Blueprint/UI/DeadUI.DeadUI_C"))
      (UserInterface|Viewport|AddtoViewport _returnvalue 0)
      (Default|PlayPlayerDeadUI _returnvalue))))

(event EventBeginPlay
  (bind _playerstats (Variables|Default|GetplayerStats))
  (bind (_maxhealth _maxoverload _basicoverloadvalue _perfectdodgeoverloadvalue _skilloverloadcost _specialattackoverloadvalue _currentattackspeed _maxattackspeed _currentcriticalchance _maxcriticalchance _currentshield _maxshield _dashcd _currentstraight _maxstraight _straightreverttime) (Utilities|Struct|BreakPlayerStats _playerstats))
  ;[1 1 1] InitData
  (Variables|HP|SetMaxHealth _maxhealth)
  (Variables|Overload|SetMaxOverload _maxoverload)
  (Variables|Overload|SetPerfect%20Dodge%20Overload%20Value _perfectdodgeoverloadvalue)
  (Variables|Overload|SetBasic%20attack%20Overload%20Value _basicoverloadvalue)
  (Variables|Overload|SetSkill%20Overload%20Cost _skilloverloadcost)
  (Variables|Overload|SetSpecial%20Attack%20Overload%20Value _specialattackoverloadvalue)
  (Variables|attackSpeed|SetmaxAttackSpeed _maxattackspeed)
  (Variables|attackSpeed|SetcurrentAttackSpeed _currentattackspeed)
  (Variables|CriticalChance|SetmaxCriticalChance _maxcriticalchance)
  (Variables|CriticalChance|SetcurrentCriticalChance _currentcriticalchance)
  (Variables|Shield|SetmaxShield _maxshield)
  (Variables|Shield|SetcurrentShield _currentshield)
  (Variables|Straight|SetcurrentStraight _currentstraight)
  (Variables|Straight|SetmaxStraight _maxstraight)
  (Variables|Straight|SetrevertStraightTime _straightreverttime))

(fn ChangeHealth
  (params (damage :type Float%20%28double-precision%29) (IncreasingType :type IncreaseEnum%20Enum :default "NewEnumerator0"))
  (bind _maxhealth (Variables|HP|GetMaxHealth))
  (if (Variables|HP|GetcanBeDamaged)
    (bind _finalstatsvalue (CallFunction|DynamicStatsChange (Variables|HP|GetCurrentHealth) _maxhealth damage IncreasingType))
    (bind _output_get (Variables|HP|SetCurrentHealth _finalstatsvalue))
    (if (<= _output_get 0.0)
      (CallFunction|SetHealthPercent _output_get _maxhealth)
      (if (not (Variables|HP|GetisPlayerDead))
        (CallFunction|PlayerDead)
        (Variables|HP|SetisPlayerDead true)
        (return true))
      (else
        (CallFunction|SetHealthPercent _output_get _maxhealth)
        (return false)))))

(fn ResetOverloadonHit
  (params (isHitByEnemy :type Boolean))
  (if isHitByEnemy
    (bind _output_get (Variables|Overload|SetCurrentOverload 0.0))
    (CallFunction|SetOverloadPercent _output_get (Variables|Overload|GetMaxOverload))))

(fn IncreaseBasicAttackOverload
  (params (isHitEnemy :type Boolean))
  (bind _maxoverload (Variables|Overload|GetMaxOverload))
  (if isHitEnemy
    (bind _finalstatsvalue (CallFunction|DynamicStatsChange (Variables|Overload|GetCurrentOverload) _maxoverload (Variables|Overload|GetBasic%20attack%20Overload%20Value) "NewEnumerator0"))
    (bind _output_get (Variables|Overload|SetCurrentOverload _finalstatsvalue))
    (CallFunction|SetOverloadPercent _output_get _maxoverload)))

(fn IncreaseOverloadonPerfectDodge
  (params (isPerfectDodge :type Boolean))
  (bind _maxoverload (Variables|Overload|GetMaxOverload))
  (if isPerfectDodge
    (bind _finalstatsvalue (CallFunction|DynamicStatsChange (Variables|Overload|GetCurrentOverload) _maxoverload (Variables|Overload|GetPerfect%20Dodge%20Overload%20Value) "NewEnumerator0"))
    (bind _output_get (Variables|Overload|SetCurrentOverload _finalstatsvalue))
    (CallFunction|SetOverloadPercent _output_get _maxoverload)))

(fn IncreaseSpecialAttackOverload
  (bind _maxoverload (Variables|Overload|GetMaxOverload))
  (bind _finalstatsvalue (CallFunction|DynamicStatsChange (Variables|Overload|GetCurrentOverload) _maxoverload (Variables|Overload|GetSpecial%20Attack%20Overload%20Value) "NewEnumerator0"))
  (bind _output_get (Variables|Overload|SetCurrentOverload _finalstatsvalue))
  (CallFunction|SetOverloadPercent _output_get _maxoverload))

(fn DynamicStatsChange
  (params (currentValue :type Float%20%28double-precision%29) (maxValue :type Float%20%28double-precision%29) (changeValue :type Float%20%28double-precision%29) (Is%20Increasing%20or%20Decreasing :type IncreaseEnum%20Enum :default "NewEnumerator0"))
  (switch Utilities|FlowControl|Switch|SwitchonIncreaseEnum Is%20Increasing%20or%20Decreasing
    (:NewEnumerator0
      (if (and (<= (+ currentValue changeValue) maxValue) (< currentValue maxValue))
        (return (+ currentValue changeValue))
        (else
          (return maxValue))))
    (:NewEnumerator1
      (if (>= (- currentValue changeValue) 0.0)
        (return (- currentValue changeValue))
        (else
          (return 0.0))))))

(fn SetHealthPercent
  (params (currentValue :type Float%20%28double-precision%29) (maxValue :type Float%20%28double-precision%29))
  (Progress|SetPercent (Variables|/Game/3_Blueprint/UI/WB_HUD.WB_HUD_C|GetHP_bar (Variables|Default|GetplayerHUD)) (/ currentValue maxValue)))

(fn SetOverloadPercent
  (params (currentValue :type Float%20%28double-precision%29) (maxValue :type Float%20%28double-precision%29))
  (Progress|SetPercent (Variables|/Game/3_Blueprint/UI/WB_HUD.WB_HUD_C|GetOverload_bar (Variables|Default|GetplayerHUD)) (/ currentValue maxValue)))

(fn ChangeAttackSpeed
  (params (IncreasedAttackSpeed :type Float%20%28double-precision%29) (IsIncreasingOrDecreasing :type IncreaseEnum%20Enum :default "NewEnumerator0"))
  (bind _finalstatsvalue (CallFunction|DynamicStatsChange (Variables|attackSpeed|GetcurrentAttackSpeed) (Variables|attackSpeed|GetmaxAttackSpeed) IncreasedAttackSpeed IsIncreasingOrDecreasing))
  (return _finalstatsvalue))

(fn ChangeCriticalChance
  (params (ChangeCriticalChance :type Float%20%28double-precision%29) (IncreaseType :type IncreaseEnum%20Enum :default "NewEnumerator0"))
  (bind _finalstatsvalue (CallFunction|DynamicStatsChange (Variables|CriticalChance|GetcurrentCriticalChance) (Variables|CriticalChance|GetmaxCriticalChance) ChangeCriticalChance IncreaseType))
  (return _finalstatsvalue))

(fn ChangeShieldValue
  (params (shieldChangeValue :type Float%20%28double-precision%29) (isIncreasingOrDecreasing :type IncreaseEnum%20Enum :default "NewEnumerator0")))

(fn ChangeStraightValue
  (params (changeValue :type Float%20%28double-precision%29))
  (bind _maxstraight (Variables|Straight|GetmaxStraight))
  (bind _output_get (Variables|Straight|SetcurrentStraight (- (Variables|Straight|GetcurrentStraight) changeValue)))
  (CallFunction|SetStraightPercent _output_get (Variables|Straight|GetmaxStraight))
  (if (not (> _output_get 0.0))
    (Animation|PlayAnimMontage (Game|GetPlayerCharacter 0) "/Game/1_Animations/Character/Hit_React/HitReactMonster_UE_Montage1.HitReactMonster_UE_Montage1" 1.0 "None")
    (Variables|Straight|SetcurrentStraight _maxstraight)
    (CallFunction|SetStraightPercent _maxstraight _maxstraight)))

(fn SetStraightPercent
  (params (currentValue :type Float%20%28double-precision%29) (maxValue :type Float%20%28double-precision%29))
  (Progress|SetPercent (Variables|/Game/3_Blueprint/UI/WB_HUD.WB_HUD_C|GetStraightBar (Variables|Default|GetplayerHUD)) (/ currentValue maxValue)))

(fn ResetStraightValue
  (bind _maxstraight (Variables|Straight|GetmaxStraight))
  (Variables|Straight|SetcurrentStraight _maxstraight)
  (CallFunction|SetStraightPercent _maxstraight _maxstraight))