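; Melee attack component for BP_TopDownCharacter, handling a three-hit sword combo and a heavy special attack.
; Attack input starts or buffers combo montages, which BasicAttackCombo continues or resets; a fourth attack is stubbed but unused.
; Heavy input cancels the combo state and chains a slow charge montage into a swing.
; A looping-timer sphere trace along the blade damages "Damageable" actors with camera shake, throttled by a delayed DoOnce reset.
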(event EventBeginPlay
  ;[1 1 1] Set the character at start
  (bind _asbp_top_down_character (Utilities|Casting|CastToBP_TopDownCharacter (Components|GetOwner)))
  (Variables|Default|SetCharacter_BP _asbp_top_down_character)
  (Variables|Default|SetCharacterMesh (Variables|/Script/Engine.Character|GetMesh _asbp_top_down_character)))

(event Custom|StopSwordTrace
  ;[1 1 1] Sword Trace
  (Utilities|Time|ClearandInvalidateTimerbyHandle (Variables|Default|GetSword%20trace%20Loop)))

(event Custom|StartSwordTrace
  ;[1 1 1] Sword Trace
  (bind _returnvalue (Utilities|Time|SetTimerbyEvent (delegate Custom|SwordTraceLoop) 0.001 true))
  (Variables|Default|SetSword%20trace%20Loop _returnvalue))

(event Custom|SwordTraceLoop
  (bind _character_bp (Variables|Default|GetCharacter_BP))
  ;[1 1 1] Sword Trace
  (bind (_outhit _returnvalue) (Collision|SphereTraceByChannel (Transformation|GetWorldLocation (Variables|/Game/Combat_XYH_WeiFu/Blueprints/BP_TopDownCharacter.BP_TopDownCharacter_C|GetSword%20Top%20Point _character_bp)) (Transformation|GetWorldLocation (Variables|/Game/Combat_XYH_WeiFu/Blueprints/BP_TopDownCharacter.BP_TopDownCharacter_C|GetSword%20Bottom%20Point _character_bp)) 12.0 "TraceTypeQuery1" false 0 "ForDuration" true "(R=1.000000,G=0.000000,B=0.000000,A=1.000000)" "(R=0.000000,G=1.000000,B=0.000000,A=1.000000)" 2.0))
  (if _returnvalue
    (if (Actor|ActorHasTag (.HitActor (Collision|BreakHitResult _outhit)) "Damageable")
      (Utilities|FlowControl|DoOnce false :!label _label
        (:Completed
          (Game|Damage|ApplyDamage (.HitActor (Collision|BreakHitResult _outhit)) (Variables|Default|GetSwordDamage) 0 0)
          (Camera|PlayWorldCameraShake "/Game/3_Blueprint/BP_SwordHitCamShake.BP_SwordHitCamShake_C" (.Location (Collision|BreakHitResult _outhit)) 0.0 2e+03)
          (Utilities|FlowControl|Delay 0.2)
          (goto _label Reset))))))

(event Custom|StopSpecialAttack
  (Variables|Default|SetisSpecialAttacking false))

(event Input|EnhancedActionEvents|EnhancedInputActionIA_HeavyAttack_State02
  (params (ActionValue :type Boolean) (ElapsedSeconds :type Float%20%28double-precision%29) (TriggeredSeconds :type Float%20%28double-precision%29) (InputAction :type Input%20Action%20Object%20Reference :default "/Game/Combat_XYH_WeiFu/Input/Actions/IA_HeavyAttack_State02.IA_HeavyAttack_State02"))
  ;[1 1 1] 重攻击蓄力阶段
)

(event Input|EnhancedActionEvents|EnhancedInputActionIA_HeavyAttack_State01
  (params (ActionValue :type Boolean) (ElapsedSeconds :type Float%20%28double-precision%29) (TriggeredSeconds :type Float%20%28double-precision%29) (InputAction :type Input%20Action%20Object%20Reference :default "/Game/Combat_XYH_WeiFu/Input/Actions/IA_HeavyAttack_State01.IA_HeavyAttack_State01"))
  ;[1 1 1] 普通重攻击
  (:Triggered
    (if (and (not (Variables|Default|GetisSpecialAttacking)) (not (Variables|Default|GetisAttacking)))
      (CallFunction|StopCombo)
      (Variables|Default|SetisSpecialAttacking true)
      (Variables|Default|SetchargingHAttackSpeed 0.5)
      (Variables|Default|SetswingHAttackSpeed 1.0)
      (Animation|Montage|PlayMontage (Variables|Default|GetCharacterMesh) "/Game/1_Animations/Character/Sword_Combat/SpecialAtttackStart.SpecialAtttackStart" (Variables|Default|GetchargingHAttackSpeed)
        (:OnBlendOut
          (Animation|Montage|PlayMontage (Variables|Default|GetCharacterMesh) "/Game/1_Animations/Character/Sword_Combat/SpecialAttackTrigger.SpecialAttackTrigger" (Variables|Default|GetswingHAttackSpeed)))))))

(event Input|EnhancedActionEvents|EnhancedInputActionIA_Heavy_Attack_State03
  (params (ActionValue :type Boolean) (ElapsedSeconds :type Float%20%28double-precision%29) (TriggeredSeconds :type Float%20%28double-precision%29) (InputAction :type Input%20Action%20Object%20Reference :default "/Game/Combat_XYH_WeiFu/Input/Actions/IA_Heavy_Attack_State03.IA_Heavy_Attack_State03"))
  ;[1 1 1] 重攻击蓄力完成阶段
)

(event Custom|BasicAttack
  ;[1 1 1] Combo System
  ;;[1 1 1] basic attack
  (if (Variables|Default|GetisAttacking)
    (Variables|Default|SetsaveAttack true)
    (else
      (Variables|Default|SetisAttacking true)
      (switch int (Variables|Default|GetattackIndex)
        (:0
          (CallFunction|Attack1))
        (:1
          (CallFunction|Attack2))
        (:2
          (CallFunction|Attack3))))))

(event Custom|BasicAttackCombo
  ;[1 1 1] Combo System
  ;;[1 1 1] Combo continue
  (if (Variables|Default|GetsaveAttack)
    (Variables|Default|SetsaveAttack false)
    (switch int (Variables|Default|GetattackIndex)
      (:0
        (CallFunction|Attack1))
      (:1
        (CallFunction|Attack2))
      (:2
        (CallFunction|Attack3)))
    (else
      (CallFunction|StopCombo))))

(event Custom|Attack_2
  ;[1 1 1] Combo System
  ;;[1 1 1] Attack_2
  (Utilities|FlowControl|DoOnce false :!label _label
    (:Completed
      (Utilities|FlowControl|Delay 0.1)
      (Animation|Montage|PlayMontage (Variables|Default|GetCharacterMesh) "/Game/1_Animations/Character/Sword_Combat/Frank_RPG_Assassin_Combo01_2_Montage.Frank_RPG_Assassin_Combo01_2_Montage" (* (Variables|Default|GetstartingAttackSpeed) (+ 1.0 (Variables|Default|GetcurrentAttackSpeed)))
        (:then
          (Variables|Default|SetattackIndex 2)
          (goto _label Reset))))))

(event Custom|Attack_3
  ;[1 1 1] Combo System
  ;;[1 1 1] Attack_3
  (Utilities|FlowControl|DoOnce false :!label _label
    (:Completed
      (Utilities|FlowControl|Delay 0.1)
      (Animation|Montage|PlayMontage (Variables|Default|GetCharacterMesh) "/Game/1_Animations/Character/Sword_Combat/Frank_RPG_Assassin_Combo01_3_Montage.Frank_RPG_Assassin_Combo01_3_Montage" (* (Variables|Default|GetstartingAttackSpeed) (+ 1.0 (Variables|Default|GetcurrentAttackSpeed)))
        (:then
          (Variables|Default|SetattackIndex 3)
          (goto _label Reset))))))

(event Custom|StopCombo
  ;[1 1 1] Combo System
  ;;[1 1 1] Stop the whole combo/attack
  (Variables|Default|SetisAttacking false)
  (Variables|Default|SetattackIndex 0))

(event Custom|Attack_4
  ;[1 1 1] Combo System
  ;;[1 1 1] Attack_4
  (Utilities|FlowControl|DoOnce false :!label _label
    (:Completed
      (Utilities|FlowControl|Delay 0.1)
      (Animation|Montage|PlayMontage (Variables|Default|GetCharacterMesh) 0 (Variables|Default|GetstartingAttackSpeed)
        (:then
          (Variables|Default|SetattackIndex 4)
          (goto _label Reset))))))

(event Custom|Attack_1
  ;[1 1 1] Combo System
  ;;[1 1 1] Attack_1
  (Utilities|FlowControl|DoOnce false :!label _label
    (:Completed
      (Animation|Montage|PlayMontage (Variables|Default|GetCharacterMesh) "/Game/1_Animations/Character/Sword_Combat/Frank_RPG_Assassin_Combo01_1_Montage.Frank_RPG_Assassin_Combo01_1_Montage" (* (Variables|Default|GetstartingAttackSpeed) (+ 1.0 (Variables|Default|GetcurrentAttackSpeed)))
        (:then
          (Variables|Default|SetattackIndex 1)
          (goto _label Reset))))))

(event Input|EnhancedActionEvents|EnhancedInputActionIA_Attack
  (params (ActionValue :type Boolean) (ElapsedSeconds :type Float%20%28double-precision%29) (TriggeredSeconds :type Float%20%28double-precision%29) (InputAction :type Input%20Action%20Object%20Reference :default "/Game/Combat_XYH_WeiFu/Input/Actions/IA_Attack.IA_Attack"))
  ;[1 1 1] Combo System
  ;;[1 1 1] Input and attack
  (:Triggered
    (if (and (Variables|Default|GetcanAttack) (not (Variables|Default|GetisSpecialAttacking)))
      (CallFunction|BasicAttack))))