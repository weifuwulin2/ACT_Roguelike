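; BPC_BlessUI is a component that manages the blessing collection prompt and blessing selection UI.
; Opening the collection prompt stores the triggering bless actor and interaction type, and closing it clears both.
; The IA_Mutually Enhanced Input action swaps the prompt for the selection widget when IsInBlessArea is true.
; A separate event destroys the stored bless actor and resets the interaction state.
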(event Custom|DestoryBlessActor
  ;[1 1 1] 销毁祝福Actor
  (Actor|DestroyActor (Variables|Default|GetTriggerBlessActor))
  (Variables|Default|SetTriggerBlessActor 0)
  (Variables|Default|SetMutuallyType "NewEnumerator4"))

(event Custom|OpenCollectionUI
  (params (BlessActor :type Actor%20Object%20Reference) (Type :type MutuallyType%20Enum :default "NewEnumerator0"))
  ;[1 1 1] 控制收集UI
  (Variables|Default|SetTriggerBlessActor BlessActor)
  (Variables|Default|SetMutuallyType Type)
  (UserInterface|Viewport|AddtoViewport (Variables|Default|GetCollectUI) 0))

(event Custom|DisableCollectionUI
  ;[1 1 1] 控制收集UI
  (Variables|Default|SetTriggerBlessActor 0)
  (Variables|Default|SetMutuallyType "NewEnumerator4")
  (Widget|RemovefromParent (Variables|Default|GetCollectUI)))

(event Custom|OpenBlessSelectUI
  ;[1 1 1] 控制祝福选择UI
  (UserInterface|Viewport|AddtoViewport (Variables|Default|GetBlessSelectUI) 0))

(event Custom|CloseBlessSelectUI
  ;[1 1 1] 控制祝福选择UI
  (Widget|RemovefromParent (Variables|Default|GetBlessSelectUI)))

(event Input|EnhancedActionEvents|EnhancedInputActionIA_Mutually
  (params (ActionValue :type Boolean) (ElapsedSeconds :type Float%20%28double-precision%29) (TriggeredSeconds :type Float%20%28double-precision%29) (InputAction :type Input%20Action%20Object%20Reference :default "/Game/Combat_XYH_WeiFu/Input/Actions/IA_Mutually.IA_Mutually"))
  ;[1 1 1] 交互键输入
  (:Triggered
    (if (Variables|Default|GetIsInBlessArea)
      (CallFunction|OpenBlessSelectUI)
      (Widget|RemovefromParent (Variables|Default|GetCollectUI)))))

(event EventBeginPlay)

(event EventTick
  (params (DeltaSeconds :type Float%20%28single-precision%29)))