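; Monster stats component that holds an enemy's health, shield, damage and attack speed.
; On BeginPlay it gets the monster key and HUD through the owner's Damageable cast, then loads health, shield and damage from DTMonsterStats.
; A shared helper handles increases, capped at max, and unclamped decreases.
; Health changes update the Enemy_Hp bar and report death, while shield and attack speed functions return results without storing them, with shield also setting the AI_Blood bar.
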(event EventBeginPlay
  ;[1 1 1] InitData
  (bind _asdamageable (Utilities|Casting|CastToDamageable (Components|GetOwner)))
  (bind _monsterkey (Default|GetMonsterKey _asdamageable))
  (bind (_defaulthp _defaultshield _defaultdamage) (CallFunction|QueryMonsterStatsUsingName _monsterkey))
  (bind _output_get (Variables|HP|SetMaxHealth _defaulthp))
  (Variables|HP|SetCurrentHealth _output_get)
  (bind _output_get_2 (Variables|Shield|SetcurrentShield _defaultshield))
  (Variables|Shield|SetmaxShield _output_get_2)
  (Variables|damage|SetcurrentDamage _defaultdamage)
  (bind _hud (Default|GetHUD _asdamageable))
  (Variables|Default|SetHUD _hud))

(event EventTick
  (params (DeltaSeconds :type Float%20%28single-precision%29)))

(fn ChangeHealth
  (params (damage :type Float%20%28double-precision%29) (IncreasingType :type IncreaseEnum%20Enum :default "NewEnumerator0"))
  (bind _maxhealth (Variables|HP|GetMaxHealth))
  (if (Variables|HP|GetcanBeDamaged)
    (bind _finalstatsvalue (CallFunction|DynamicStatsChange (Variables|HP|GetCurrentHealth) _maxhealth damage IncreasingType))
    (bind _output_get (Variables|HP|SetCurrentHealth _finalstatsvalue))
    (if (<= _output_get 0.0)
      (CallFunction|SetHealthPercent _output_get _maxhealth)
      (return true)
      (else
        (CallFunction|SetHealthPercent _output_get _maxhealth)
        (return false)))))

(fn DynamicStatsChange
  (params (currentValue :type Float%20%28double-precision%29) (maxValue :type Float%20%28double-precision%29) (changeValue :type Float%20%28double-precision%29) (Is%20Increasing%20or%20Decreasing :type IncreaseEnum%20Enum :default "NewEnumerator0"))
  (switch Utilities|FlowControl|Switch|SwitchonIncreaseEnum Is%20Increasing%20or%20Decreasing
    (:NewEnumerator0
      (if (and (<= (+ currentValue changeValue) maxValue) (< currentValue maxValue))
        (return (+ currentValue changeValue))
        (else
          (return maxValue))))
    (:NewEnumerator1
      (return (- currentValue changeValue)))))

(fn SetHealthPercent
  (params (currentValue :type Float%20%28double-precision%29) (maxValue :type Float%20%28double-precision%29))
  (bind _asenemy_hp (Utilities|Casting|CastToEnemy_Hp (UserInterface|GetWidget (Variables|Default|GetHUD))))
  (Progress|SetPercent (Variables|/Game/Combat_XYH_WeiFu/Enemies/UI/Enemy_Hp.Enemy_Hp_C|GetHP_bar _asenemy_hp) (/ currentValue maxValue)))

(fn ChangeAttackSpeed
  (params (IncreasedAttackSpeed :type Float%20%28double-precision%29) (IsIncreasingOrDecreasing :type IncreaseEnum%20Enum :default "NewEnumerator0"))
  (bind _finalstatsvalue (CallFunction|DynamicStatsChange (Variables|AttackSpeed|GetcurrentAttackSpeed) (Variables|attackSpeed|GetmaxAttackSpeed) IncreasedAttackSpeed IsIncreasingOrDecreasing))
  (return _finalstatsvalue))

(fn ChangeShieldValue
  (params (shieldChangeValue :type Float%20%28double-precision%29) (isIncreasingOrDecreasing :type IncreaseEnum%20Enum :default "NewEnumerator0"))
  (bind _finalstatsvalue (CallFunction|DynamicStatsChange (Variables|Shield|GetcurrentShield) (Variables|Shield|GetmaxShield) shieldChangeValue isIncreasingOrDecreasing))
  (bind _asai_blood (Utilities|Casting|CastToAI_Blood (UserInterface|GetUserWidgetObject (Variables|Default|GetHUD))))
  (Progress|SetPercent (Variables|/Game/Cyborg_soldier_V1_ShaoZhiGao/Enemy_AI/AI/AI_Blood.AI_Blood_C|GetShieldBar _asai_blood) _finalstatsvalue)
  (return _finalstatsvalue))

(fn QueryMonsterStatsUsingName
  (params (Key :type Name))
  (bind _dt_monsterstats (Variables|Default|GetDT_MonsterStats))
  (bind _outrownames (DataTable|GetDataTableRowNames _dt_monsterstats))
  (for _array_element _outrownames
    (if (== Key _array_element)
      (bind _returnvalue (Utilities|GetDataTableRow _dt_monsterstats Key)
        (:then
          (return (.maxHealth (Utilities|Struct|BreakStruct_MonsterStats _returnvalue)) (.maxShield (Utilities|Struct|BreakStruct_MonsterStats _returnvalue)) (.damage (Utilities|Struct|BreakStruct_MonsterStats _returnvalue))))))))

(fn ChangeCurrentDamage
  (params (newDamage :type Float%20%28double-precision%29))
  (bind _output_get (Variables|damage|SetcurrentDamage newDamage))
  (return _output_get))