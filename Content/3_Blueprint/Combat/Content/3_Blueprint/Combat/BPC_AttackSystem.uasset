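; Player attack component for BP_TopDownCharacter, handling melee combos, a charged heavy attack and sword hit detection.
; Basic attacks buffer input to chain three data-table montages scaled by attack speed; a parallel special combo has its trigger disconnected.
; Heavy attack holds a charge montage with curve-driven play rate and camera shake.
; A timer-looped sphere trace hits each Damageable once, triggering damage calls, overload gain and hit-stop, sound, VFX and shake feedback.
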(event Custom|StopSwordTrace
  ;[1 1 1] Sword Trace
  (Utilities|Time|ClearandInvalidateTimerbyHandle (Variables|BasicAttack|GetSword%20trace%20Loop))
  (Utilities|Array|Clear (Variables|BasicAttack|GetHit%20Actors)))

(event Custom|DunFrame
  (params (Duration :type Float%20%28double-precision%29) (LastTime :type Float%20%28double-precision%29))
  ;[1 1 1] 顿帧
  (Utilities|Time|SetGlobalTimeDilation Duration)
  (Utilities|FlowControl|RetriggerableDelay LastTime)
  (Utilities|Time|SetGlobalTimeDilation 1.0))

(event Custom|ComBatFeedback
  (params (HitLocation :type Vector) (Feedback :type Feedback%20Structure))
  ;[1 1 1] 封装好的反馈
  (Audio|PlaySound2D (.hit_sfx Feedback) 1.0 1.0 0.12 0 0 false) ; 这里后面要修音效
  (Niagara|SpawnSystematLocation (.hit_fx Feedback) HitLocation)
  (CallFunction|DunFrame (.dunframeduration Feedback) (.dunframetime Feedback))
  (Camera|PlayWorldCameraShake (.shakeconfig Feedback) HitLocation 0.0 2e+03))

(event Custom|StartSwordTrace
  (params (HitFeedback :type Feedback%20Structure))
  ;[1 1 1] Sword Trace
  (Variables|BasicAttack|SetHitFeedbackConfig HitFeedback)
  (bind _returnvalue (Utilities|Time|SetTimerbyEvent (delegate Custom|SwordTraceLoop) 0.001 true))
  (Variables|BasicAttack|SetSword%20trace%20Loop _returnvalue))

(event Custom|SwordTraceLoop
  (bind _character_bp (Variables|References|GetCharacter_BP))
  (bind _hit_actors (Variables|BasicAttack|GetHit%20Actors))
  ;[1 1 1] Sword Trace
  (bind (_outhit _returnvalue) (Collision|SphereTraceByChannel (Transformation|GetWorldLocation (Variables|/Game/Combat_XYH_WeiFu/Blueprints/BP_TopDownCharacter.BP_TopDownCharacter_C|GetSword%20Top%20Point _character_bp)) (Transformation|GetWorldLocation (Variables|/Game/Combat_XYH_WeiFu/Blueprints/BP_TopDownCharacter.BP_TopDownCharacter_C|GetSword%20Bottom%20Point _character_bp)) 12.0 "TraceTypeQuery1" false 0 "Persistent" true "(R=1.000000,G=0.000000,B=0.000000,A=1.000000)" "(R=0.000000,G=1.000000,B=0.000000,A=1.000000)" 2.0))
  (if _returnvalue
    (Utilities|Casting|CastToDamageable (.HitActor (Collision|BreakHitResult _outhit)))
    (if (not (Utilities|Array|ContainsItem _hit_actors (.HitActor (Collision|BreakHitResult _outhit))))
      (CallFunction|ComBatFeedback (.Location (Collision|BreakHitResult _outhit)) (Variables|BasicAttack|GetHitFeedbackConfig))
      (Utilities|Array|Add _hit_actors (.HitActor (Collision|BreakHitResult _outhit)))
      (bind _asdamageable (Utilities|Casting|CastToDamageable (.HitActor (Collision|BreakHitResult _outhit))))
      (bind _asbp_top_down_character (Utilities|Casting|CastToBP_TopDownCharacter (Game|GetPlayerCharacter 0)))
      (bind _monsterstats (Default|GetMonsterStats _asdamageable))
      (Default|CalculateDamage (Variables|/Game/Combat_XYH_WeiFu/Blueprints/BP_TopDownCharacter.BP_TopDownCharacter_C|GetBPC_DamageCalculation _asbp_top_down_character) (Variables|BasicAttack|GetattackDamage) (Variables|/Game/3_Blueprint/PlayerStats/BPC_PlayerStats.BPC_PlayerStats_C|GetcurrentCriticalChance (Variables|/Game/Combat_XYH_WeiFu/Blueprints/BP_TopDownCharacter.BP_TopDownCharacter_C|GetBPC_PlayerStats _asbp_top_down_character)))
      (Default|ChangeHealth _asdamageable _monsterstats 0.0 "NewEnumerator0")
      (Default|GetHit _asdamageable)
      (bind _asbp_top_down_character_2 (Utilities|Casting|CastToBP_TopDownCharacter (Game|GetPlayerCharacter 0)))
      (Default|IncreaseBasicAttackOverload (Variables|/Game/Combat_XYH_WeiFu/Blueprints/BP_TopDownCharacter.BP_TopDownCharacter_C|GetBPC_PlayerStats _asbp_top_down_character_2) false))))

(event EventBeginPlay
  ;[1 1 1] Set the character at start
  (Utilities|FlowControl|Sequence
    (:then_0
      (bind _asbp_top_down_character (Utilities|Casting|CastToBP_TopDownCharacter (Components|GetOwner)))
      (Variables|References|SetCharacter_BP _asbp_top_down_character)
      (Variables|References|SetCharacterMesh (Variables|/Script/Engine.Character|GetMesh _asbp_top_down_character))
      (Variables|References|SetcameraShakeSource (Variables|/Game/Combat_XYH_WeiFu/Blueprints/BP_TopDownCharacter.BP_TopDownCharacter_C|GetCameraShakeSource _asbp_top_down_character))
      (Variables|References|SetBPC%20Player%20Stats (Variables|/Game/Combat_XYH_WeiFu/Blueprints/BP_TopDownCharacter.BP_TopDownCharacter_C|GetBPC_PlayerStats _asbp_top_down_character)))))

(fn GetCurrentAttackSpeed
  (return (Variables|/Game/3_Blueprint/PlayerStats/BPC_PlayerStats.BPC_PlayerStats_C|GetcurrentAttackSpeed (Variables|References|GetBPC%20Player%20Stats))))

(fn GetBasicAttackMontagefromDT
  (params (key :type Name))
  (bind _dt_basicattack (Variables|BasicAttack|GetDT_BasicAttack))
  (bind _outrownames (DataTable|GetDataTableRowNames _dt_basicattack))
  (for _array_element _outrownames
    (if (== key _array_element)
      (bind _returnvalue (Utilities|GetDataTableRow _dt_basicattack key)
        (:then
          (return (.montageReference (Utilities|Struct|BreakStruct_BasicAttacks _returnvalue)) (.damage (Utilities|Struct|BreakStruct_BasicAttacks _returnvalue))))))))

(fn GetSpecialAttackMontagefromDT
  (params (key :type Name))
  (bind _dtspecialattack (Variables|SPAttack|GetDTSpecialAttack))
  (bind _outrownames (DataTable|GetDataTableRowNames _dtspecialattack))
  (for _array_element _outrownames
    (if (== key _array_element)
      (bind _returnvalue (Utilities|GetDataTableRow _dtspecialattack key)
        (:then
          (return (.montageReference (Utilities|Struct|BreakStruct_BasicAttacks _returnvalue))))))))

(event Custom|BaseSPAttack
  ;[1 1 1] 特攻连招派生
  ;;[1 1 1] basic attack
  (if (Variables|SPAttack|GetisSPAttacking)
    (Variables|SPAttack|SetsaveSPAttack true)
    (else
      (Variables|SPAttack|SetisSPAttacking true)
      (switch int (Variables|SPAttack|GetSPAttackIndex)
        (:0
          (CallFunction|SPAttack1))
        (:1
          (CallFunction|SPAttack2))
        (:2
          (CallFunction|SPAttack3))))))

(event Custom|BaseSPAttackCombo
  ;[1 1 1] 特攻连招派生
  ;;[1 1 1] Combo continue
  (if (Variables|SPAttack|GetsaveSPAttack)
    (Variables|SPAttack|SetsaveSPAttack false)
    (switch int (Variables|SPAttack|GetSPAttackIndex)
      (:0
        (CallFunction|SPAttack1))
      (:1
        (CallFunction|SPAttack2))
      (:2
        (CallFunction|SPAttack3)))
    (else
      (CallFunction|StopSPAttackCombo))))

(event Custom|SPAttack2
  ;[1 1 1] 特攻连招派生
  ;;[1 1 1] Attack_2
  (Utilities|FlowControl|DoOnce false :!label _label
    (:Completed
      (bind _currentattackspeed (CallFunction|GetCurrentAttackSpeed))
      (Animation|Montage|PlayMontage (Variables|References|GetCharacterMesh) "/Game/1_Animations/Character/Sword_Combat/Base_Attack_Combo_2_Montage.Base_Attack_Combo_2_Montage" (* (Variables|BasicAttack|GetstartingAttackSpeed) (+ 1.0 _currentattackspeed))
        (:then
          (Variables|SPAttack|SetSPAttackIndex 2)
          (goto _label Reset))))))

(event Custom|SPAttack3
  ;[1 1 1] 特攻连招派生
  ;;[1 1 1] Attack_3
  (Utilities|FlowControl|DoOnce false :!label _label
    (:Completed
      (bind _currentattackspeed (CallFunction|GetCurrentAttackSpeed))
      (Animation|Montage|PlayMontage (Variables|References|GetCharacterMesh) "/Game/1_Animations/Character/Sword_Combat/Base_Attack_Combo_3_Montage.Base_Attack_Combo_3_Montage" (* (Variables|BasicAttack|GetstartingAttackSpeed) (+ 1.0 _currentattackspeed))
        (:then
          (Variables|SPAttack|SetSPAttackIndex 3)
          (goto _label Reset))))))

(event Custom|StopSPAttackCombo
  ;[1 1 1] 特攻连招派生
  ;;[1 1 1] Stop the whole combo/attack
  (Variables|SPAttack|SetisSPAttacking false)
  (Variables|SPAttack|SetSPAttackIndex 0))

(event Custom|stopSPChargeAttack
  ;[1 1 1] 蓄力特攻派生
  (Variables|SPAttack|SetisSPChargeAttacking false))

(event Custom|SPAttack4
  ;[1 1 1] 特攻连招派生
  ;;[1 1 1] Attack_4
  (Utilities|FlowControl|DoOnce false :!label _label
    (:Completed
      (bind _currentattackspeed (CallFunction|GetCurrentAttackSpeed))
      (Animation|Montage|PlayMontage (Variables|References|GetCharacterMesh) 0 (Variables|BasicAttack|GetstartingAttackSpeed)
        (:then
          (Variables|SPAttack|SetSPAttackIndex 4)
          (goto _label Reset))))))

(event Custom|SPAttack1
  ;[1 1 1] 特攻连招派生
  ;;[1 1 1] Attack_1
  (Utilities|FlowControl|DoOnce false :!label _label
    (:Completed
      (bind _currentattackspeed (CallFunction|GetCurrentAttackSpeed))
      (Animation|Montage|PlayMontage (Variables|References|GetCharacterMesh) "/Game/1_Animations/Character/Sword_Combat/Base_Attack_Combo_1_Montage.Base_Attack_Combo_1_Montage" (* (Variables|BasicAttack|GetstartingAttackSpeed) (+ 1.0 _currentattackspeed))
        (:then
          (Variables|SPAttack|SetSPAttackIndex 1)
          (goto _label Reset))))))

(event Input|EnhancedActionEvents|EnhancedInputActionIA_HeavyAttack_State01
  (params (ActionValue :type Boolean) (ElapsedSeconds :type Float%20%28double-precision%29) (TriggeredSeconds :type Float%20%28double-precision%29) (InputAction :type Input%20Action%20Object%20Reference :default "/Game/Combat_XYH_WeiFu/Input/Actions/IA_HeavyAttack_State01.IA_HeavyAttack_State01"))
  ;[1 1 1] 特攻连招派生
  ;;[1 1 1] Input and attack
)

(event Input|EnhancedActionEvents|EnhancedInputActionIA_HeavyAttack_State02
  (params (ActionValue :type Boolean) (ElapsedSeconds :type Float%20%28double-precision%29) (TriggeredSeconds :type Float%20%28double-precision%29) (InputAction :type Input%20Action%20Object%20Reference :default "/Game/Combat_XYH_WeiFu/Input/Actions/IA_HeavyAttack_State02.IA_HeavyAttack_State02"))
  (bind _charactermesh (Variables|References|GetCharacterMesh))
  (bind _returnvalue (Components|SkeletalMesh|GetAnimInstance _charactermesh))
  ;[1 1 1] 蓄力特攻派生
  (:Triggered
    (if (not (Variables|BasicAttack|GetisAttacking))
      (Utilities|FlowControl|DoOnce true :!label _label
        (:Completed
          (bind _anim_montage_found (CallFunction|GetSpecialAttackMontagefromDT "SpecialAttack_0"))
          (Animation|Montage|PlayMontage (Variables|References|GetCharacterMesh) _anim_montage_found 1.0 0.0 "ChargeSuccess")))))
  (:Started
    (if (Math|Boolean|ANDBoolean (Variables|SPAttack|GetcanSPAttack) (not (Variables|BasicAttack|GetisAttacking)) (not (Variables|SPAttack|GetisSPChargeAttacking)))
      (Development|PrintString "播放动画")
      (Variables|SPAttack|SetisSPChargeAttacking true)
      (bind _anim_montage_found_2 (CallFunction|GetSpecialAttackMontagefromDT "SpecialAttack_0"))
      (Animation|Montage|PlayMontage (Variables|References|GetCharacterMesh) _anim_montage_found_2 1.0 0.0 ""
        (:OnCompleted
          _)
        (:OnBlendOut
          _)
        (:OnInterrupted
          _)
        (:OnNotifyBegin
          (CameraShakes|StartCameraShake (Variables|References|GetcameraShakeSource) "/Game/3_Blueprint/Combat/BP_SP_HoldCamShake.BP_SP_HoldCamShake_C" 1.0 "CameraLocal" "0, 0, 0")
          (Utilities|FlowControl|Sequence
            (:then_0
              (goto _label_2 Reset))
            (:then_1
              (goto _label Reset)))))
      (CameraShake|StopAllCameraShakes (Variables|References|GetcameraShakeSource) true)))
  (:Ongoing
    (if (not (Variables|BasicAttack|GetisAttacking))
      (Animation|Montage|MontageSetPlayRate _returnvalue 0 (Animation|Curves|GetCurveValue _returnvalue "ChargeAttack"))
      (if (>= ElapsedSeconds 1.0)
        (Utilities|FlowControl|DoOnce true :!label _label_2
          (:Completed
            (Niagara|SpawnSystematLocation "/Game/2_Assets/StrikeVFX/FX/FX_ReaperStrike.FX_ReaperStrike" (Transformation|GetActorLocation (Variables|References|GetCharacter_BP))))))))
  (:Canceled
    (Animation|Montage|MontageStop (Components|SkeletalMesh|GetAnimInstance (Variables|References|GetCharacterMesh)) 0.5 "/Game/1_Animations/Character/Sword_Combat/SP_Attack_ChargeAttack_Montage.SP_Attack_ChargeAttack_Montage")
    (Default|MountWeapon (Variables|/Game/Combat_XYH_WeiFu/Blueprints/BP_TopDownCharacter.BP_TopDownCharacter_C|GetBPC_WeaponSystem (Variables|References|GetCharacter_BP)))
    (CallFunction|StopSPChargeAttack)))

(event Custom|BasicAttack
  ;[1 1 1] Combo System
  ;;[1 1 1] basic attack
  (if (Variables|BasicAttack|GetisAttacking)
    (Variables|BasicAttack|SetsaveAttack true)
    (else
      (Variables|BasicAttack|SetisAttacking true)
      (switch int (Variables|BasicAttack|GetattackIndex)
        (:0
          (CallFunction|Attack1))
        (:1
          (CallFunction|Attack2))
        (:2
          (CallFunction|Attack3))))))

(event Custom|BasicAttackCombo
  ;[1 1 1] Combo System
  ;;[1 1 1] Combo continue
  (if (Variables|BasicAttack|GetsaveAttack)
    (Variables|BasicAttack|SetsaveAttack false)
    (switch int (Variables|BasicAttack|GetattackIndex)
      (:0
        (CallFunction|Attack1))
      (:1
        (CallFunction|Attack2))
      (:2
        (CallFunction|Attack3)))
    (else
      (CallFunction|StopCombo))))

(event Custom|Attack_2
  ;[1 1 1] Combo System
  ;;[1 1 1] Attack_2
  (Utilities|FlowControl|DoOnce false :!label _label
    (:Completed
      (bind _currentattackspeed (CallFunction|GetCurrentAttackSpeed))
      (bind (_anim_montage_found _damage) (CallFunction|GetBasicAttackMontagefromDT "basicAttack_1"))
      (Variables|BasicAttack|SetattackDamage _damage)
      (Animation|Montage|PlayMontage (Variables|References|GetCharacterMesh) _anim_montage_found (* (Variables|BasicAttack|GetstartingAttackSpeed) (+ 1.0 _currentattackspeed))
        (:then
          (Variables|BasicAttack|SetattackIndex 2)
          (goto _label Reset))))))

(event Custom|Attack_3
  ;[1 1 1] Combo System
  ;;[1 1 1] Attack_3
  (Utilities|FlowControl|DoOnce false :!label _label
    (:Completed
      (bind _currentattackspeed (CallFunction|GetCurrentAttackSpeed))
      (bind (_anim_montage_found _damage) (CallFunction|GetBasicAttackMontagefromDT "basicAttack_2"))
      (Variables|BasicAttack|SetattackDamage _damage)
      (Animation|Montage|PlayMontage (Variables|References|GetCharacterMesh) _anim_montage_found (* (Variables|BasicAttack|GetstartingAttackSpeed) (+ 1.0 _currentattackspeed))
        (:then
          (Variables|BasicAttack|SetattackIndex 3)
          (goto _label Reset))))))

(event Custom|StopCombo
  ;[1 1 1] Combo System
  ;;[1 1 1] Stop the whole combo/attack
  (Variables|BasicAttack|SetisAttacking false)
  (Variables|BasicAttack|SetattackIndex 0))

(event Custom|Attack_4
  ;[1 1 1] Combo System
  ;;[1 1 1] Attack_4
  (Utilities|FlowControl|DoOnce false :!label _label
    (:Completed
      (bind _currentattackspeed (CallFunction|GetCurrentAttackSpeed))
      (Animation|Montage|PlayMontage (Variables|References|GetCharacterMesh) 0 (Variables|BasicAttack|GetstartingAttackSpeed)
        (:then
          (Variables|BasicAttack|SetattackIndex 4)
          (goto _label Reset))))))

(event Custom|Attack_1
  ;[1 1 1] Combo System
  ;;[1 1 1] Attack_1
  (Utilities|FlowControl|DoOnce false :!label _label
    (:Completed
      (bind _currentattackspeed (CallFunction|GetCurrentAttackSpeed))
      (bind (_anim_montage_found _damage) (CallFunction|GetBasicAttackMontagefromDT "basicAttack_0"))
      (Variables|BasicAttack|SetattackDamage _damage)
      (Animation|Montage|PlayMontage (Variables|References|GetCharacterMesh) _anim_montage_found (* (Variables|BasicAttack|GetstartingAttackSpeed) (+ 1.0 _currentattackspeed))
        (:then
          (Variables|BasicAttack|SetattackIndex 1)
          (goto _label Reset))))))

(event Input|EnhancedActionEvents|EnhancedInputActionIA_Attack
  (params (ActionValue :type Boolean) (ElapsedSeconds :type Float%20%28double-precision%29) (TriggeredSeconds :type Float%20%28double-precision%29) (InputAction :type Input%20Action%20Object%20Reference :default "/Game/Combat_XYH_WeiFu/Input/Actions/IA_Attack.IA_Attack"))
  (bind _character_bp (Variables|References|GetCharacter_BP))
  (bind _bpc_dashattack (Variables|/Game/Combat_XYH_WeiFu/Blueprints/BP_TopDownCharacter.BP_TopDownCharacter_C|GetBPC_DashAttack _character_bp))
  ;[1 1 1] Combo System
  ;;[1 1 1] Input and attack
  (:Triggered
    (if (Variables|/Game/3_Blueprint/Combat/BPC_DashAttack.BPC_DashAttack_C|GetisDashing _bpc_dashattack)
      (Variables|/Game/3_Blueprint/Combat/BPC_DashAttack.BPC_DashAttack_C|SetcanAttackDash _bpc_dashattack true)
      (elif (Variables|BasicAttack|GetcanAttack)
        (CallFunction|BasicAttack)))))