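; Dash attack component for BP_TopDownCharacter, triggered by the IA_Dash input action.
; On dash it plays the DashAttack00 montage, stores the owner's forward vector, and restarts the character's DashTimeLine with callbacks bound at runtime.
; Each timeline update sets movement velocity along that stored direction, scaled by the character's DashDistanceMul and Distance.
; The finish callback is empty, and no hit or damage logic lives here.
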(event Custom|Dash
  (bind _as_bp_top_down_character (Variables|Default|GetAs%20BP%20Top%20Down%20Character))
  (bind _as_bp_top_down_character_2 (Variables|Default|GetAs%20BP%20Top%20Down%20Character))
  (bind _dashtimeline (Variables|/Game/Combat_XYH_WeiFu/Blueprints/BP_TopDownCharacter.BP_TopDownCharacter_C|GetDashTimeLine _as_bp_top_down_character_2))
  (Animation|PlayAnimMontage _as_bp_top_down_character "/Game/1_Animations/Character/Dash/DashAttack00_Montage.DashAttack00_Montage" 1.0 "None")
  (bind _output_get (Variables|Default|SetVectorValue (Transformation|GetActorForwardVector _as_bp_top_down_character)))
  (Class|TimelineComponent|SetTimelinePostUpdateFunc _dashtimeline (delegate Custom|DashUpdate))
  (Class|TimelineComponent|SetTimelineFinishedFunc _dashtimeline (delegate Custom|DashEnd))
  (Components|Timeline|PlayfromStart _dashtimeline))

(event Custom|DashUpdate
  (Variables|/Script/Engine.MovementComponent|SetVelocity (Variables|/Script/Engine.Character|GetCharacterMovement (Variables|Default|GetAs%20BP%20Top%20Down%20Character)) (* (stale Custom|Dash _output_get) (* (Variables|/Game/Combat_XYH_WeiFu/Blueprints/BP_TopDownCharacter.BP_TopDownCharacter_C|GetDashDistanceMul (Variables|Default|GetAs%20BP%20Top%20Down%20Character)) (Variables|Default|GetDistance)))))

(event Custom|DashEnd)

(event Input|EnhancedActionEvents|EnhancedInputActionIA_Dash
  (params (ActionValue :type Boolean) (ElapsedSeconds :type Float%20%28double-precision%29) (TriggeredSeconds :type Float%20%28double-precision%29) (InputAction :type Input%20Action%20Object%20Reference :default "/Game/Combat_XYH_WeiFu/Input/Actions/IA_Dash.IA_Dash"))
  (CallFunction|Dash))

(event EventBeginPlay
  (bind _asbp_top_down_character (Utilities|Casting|CastToBP_TopDownCharacter (Components|GetOwner)))
  (Variables|Default|SetCharacter%20Mesh (Variables|/Script/Engine.Character|GetMesh _asbp_top_down_character))
  (Variables|Default|SetAs%20BP%20Top%20Down%20Character _asbp_top_down_character))