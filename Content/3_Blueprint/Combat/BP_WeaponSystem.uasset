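; BP_WeaponSystem switches the player's weapon between mounted and in-hand display.
; Its MountWeapon and HandWeapon events each cast player character 0 to BP_TopDownCharacter and toggle that character's HandWeapon and MountWeapon components so only one is visible.
; Visibility changes do not propagate to child components, and each event prints a debug string.
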(event Custom|MountWeapon
  ;[1 1 1] 挂载武器逻辑
  (Development|PrintString "挂载武器")
  (bind _asbp_top_down_character (Utilities|Casting|CastToBP_TopDownCharacter (Game|GetPlayerCharacter 0)))
  (Rendering|SetVisibility (Variables|/Game/Combat_XYH_WeiFu/Blueprints/BP_TopDownCharacter.BP_TopDownCharacter_C|GetHandWeapon _asbp_top_down_character) false false)
  (Rendering|SetVisibility (Variables|/Game/Combat_XYH_WeiFu/Blueprints/BP_TopDownCharacter.BP_TopDownCharacter_C|GetMountWeapon _asbp_top_down_character) true false))

(event Custom|HandWeapon
  ;[1 1 1] 手持武器逻辑
  (Development|PrintString "手持武器")
  (bind _asbp_top_down_character (Utilities|Casting|CastToBP_TopDownCharacter (Game|GetPlayerCharacter 0)))
  (Rendering|SetVisibility (Variables|/Game/Combat_XYH_WeiFu/Blueprints/BP_TopDownCharacter.BP_TopDownCharacter_C|GetHandWeapon _asbp_top_down_character) true false)
  (Rendering|SetVisibility (Variables|/Game/Combat_XYH_WeiFu/Blueprints/BP_TopDownCharacter.BP_TopDownCharacter_C|GetMountWeapon _asbp_top_down_character) false false))