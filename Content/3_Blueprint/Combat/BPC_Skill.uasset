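; Player skill component with an overload-driven passive and an input-triggered active skill.
; BeginPlay caches the player state, damage calculation and attack system components from BP_TopDownCharacter.
; Every Tick, full CurrentOverload applies damage and attack speed multipliers, otherwise both are reset to normal.
; IA_Skill checks the same overload threshold but only prints a success message, with no skill effect or overload cost.
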(event Input|EnhancedActionEvents|EnhancedInputActionIA_Skill
  (params (ActionValue :type Boolean) (ElapsedSeconds :type Float%20%28double-precision%29) (TriggeredSeconds :type Float%20%28double-precision%29) (InputAction :type Input%20Action%20Object%20Reference :default "/Game/Combat_XYH_WeiFu/Input/Actions/IA_Skill.IA_Skill"))
  ;[1 1 1] 主动
  (:Triggered
    (if (>= (Variables|/Game/3_Blueprint/PlayerStats/BPC_PlayerStats.BPC_PlayerStats_C|GetCurrentOverload (Variables|Default|GetBPC_PlayerState)) 1e+02)
      (Development|PrintString "释放技能成功"))))

(event EventBeginPlay
  ;[1 1 1] 初始化变量
  (bind _asbp_top_down_character (Utilities|Casting|CastToBP_TopDownCharacter (Game|GetPlayerCharacter 0)))
  (Variables|Default|SetBPC_PlayerState (Variables|/Game/Combat_XYH_WeiFu/Blueprints/BP_TopDownCharacter.BP_TopDownCharacter_C|GetBPC_PlayerStats _asbp_top_down_character))
  (Variables|Default|SetBPC_DamageCal (Variables|/Game/Combat_XYH_WeiFu/Blueprints/BP_TopDownCharacter.BP_TopDownCharacter_C|GetBPC_DamageCalculation _asbp_top_down_character))
  (Variables|Default|SetBPC_AttackSystem (Variables|/Game/Combat_XYH_WeiFu/Blueprints/BP_TopDownCharacter.BP_TopDownCharacter_C|GetBPC_AttackSystem _asbp_top_down_character)))

(event EventTick
  (params (DeltaSeconds :type Float%20%28single-precision%29))
  ;[1 1 1] 被动
  (if (>= (Variables|/Game/3_Blueprint/PlayerStats/BPC_PlayerStats.BPC_PlayerStats_C|GetCurrentOverload (Variables|Default|GetBPC_PlayerState)) 1e+02)
    (Development|PrintString "触发被动效果")
    (Variables|/Game/3_Blueprint/Combat/BPC_DamageCalculation.BPC_DamageCalculation_C|SetExtraDmg (Variables|Default|GetBPC_DamageCal) 1.2)
    (Variables|/Game/3_Blueprint/Combat/BPC_AttackSystem.BPC_AttackSystem_C|SetstartingAttackSpeed (Variables|Default|GetBPC_AttackSystem) 1.3)
    (else
      (Variables|/Game/3_Blueprint/Combat/BPC_DamageCalculation.BPC_DamageCalculation_C|SetExtraDmg (Variables|Default|GetBPC_DamageCal) 1.0)
      (Variables|/Game/3_Blueprint/Combat/BPC_AttackSystem.BPC_AttackSystem_C|SetstartingAttackSpeed (Variables|Default|GetBPC_AttackSystem) 1.0))))