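; Actor component that handles the dash and dash attack for BP_TopDownCharacter.
; IA_Dash sets IsDashing, blocks the attack system's CanAttack and plays a dash montage with sound, using DoOnce and DashCD delays.
; StopDashAttack restores both flags, while DashAttackCombo re-enters the dash directly.
; Tick polls CanAttackDash to fire a cooldown-gated DashAttack, and Dash_Attack plays a combo montage after a short delay.
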(event EventTick
  (params (DeltaSeconds :type Float%20%28single-precision%29)))

(event EventBeginPlay
  (bind _asbp_top_down_character (Utilities|Casting|CastToBP_TopDownCharacter (Components|GetOwner)))
  (Variables|Default|SetCharacter%20Mesh (Variables|/Script/Engine.Character|GetMesh _asbp_top_down_character))
  (Variables|Default|SetAs%20BP%20Top%20Down%20Character _asbp_top_down_character))

(event Custom|DashAttackDetection
  ;[1 1 1] basic attack
  (if (not (Variables|Default|GetisDashing))
    (Variables|Default|SetisDashing true)
    (Variables|/Game/3_Blueprint/Combat/BPC_AttackSystem.BPC_AttackSystem_C|SetcanAttack (Variables|/Game/Combat_XYH_WeiFu/Blueprints/BP_TopDownCharacter.BP_TopDownCharacter_C|GetBPC_AttackSystem (Variables|Default|GetAs%20BP%20Top%20Down%20Character)) false)
    ;[1 1 1] Combo continue
    (CallFunction|NormalDash)))

(event Custom|DashAttackCombo
  ;[1 1 1] Combo continue
  (CallFunction|NormalDash))

(event Custom|StopDashAttack
  ;[1 1 1] Stop the whole combo/attack
  (Variables|Default|SetisDashing false)
  (Variables|/Game/3_Blueprint/Combat/BPC_AttackSystem.BPC_AttackSystem_C|SetcanAttack (Variables|/Game/Combat_XYH_WeiFu/Blueprints/BP_TopDownCharacter.BP_TopDownCharacter_C|GetBPC_AttackSystem (Variables|Default|GetAs%20BP%20Top%20Down%20Character)) true))

(event Custom|Dash_Attack
  ;[1 1 1] DashAttack_0
  (Utilities|FlowControl|DoOnce false :!label _label
    (:Completed
      (Utilities|FlowControl|Delay 0.1)
      (Animation|Montage|PlayMontage (Variables|Default|GetCharacter%20Mesh) "/Game/1_Animations/Character/Dash/Frank_RPG_Assassin_Combo04_1_Montage.Frank_RPG_Assassin_Combo04_1_Montage"
        (:then
          (goto _label Reset))))))

(event Custom|NormalDash
  (bind _dash_cd (Variables|Default|GetDash%20CD))
  ;[1 1 1] NormalDash
  (Utilities|FlowControl|Sequence
    (:then_0
      (Utilities|FlowControl|DoOnce false :!label _label
        (:Completed
          (Animation|Montage|PlayMontage (Variables|Default|GetCharacter%20Mesh) "/Game/1_Animations/Character/Dash/FemaleLocomotionPose_UE_Montage.FemaleLocomotionPose_UE_Montage"
            (:then
              (Utilities|FlowControl|Sequence
                (:then_0
                  (Utilities|FlowControl|Delay _dash_cd))
                (:then_1
                  (Audio|PlaySound2D 0 1.0 1.0 0.0 0 0)
                  (Utilities|FlowControl|Delay _dash_cd)
                  (goto _label Reset))))))))))

(event Input|EnhancedActionEvents|EnhancedInputActionIA_Dash
  (params (ActionValue :type Boolean) (ElapsedSeconds :type Float%20%28double-precision%29) (TriggeredSeconds :type Float%20%28double-precision%29) (InputAction :type Input%20Action%20Object%20Reference :default "/Game/Combat_XYH_WeiFu/Input/Actions/IA_Dash.IA_Dash"))
  (:Triggered
    (CallFunction|DashAttackDetection)))

(event EventTick
  (params (DeltaSeconds :type Float%20%28single-precision%29))
  (if (Variables|Default|GetcanAttackDash)
    (Utilities|FlowControl|DoOnce false :!label _label
      (:Completed
        (CallFunction|DashAttack)
        (Variables|Default|SetcanAttackDash false)
        (Utilities|FlowControl|Delay (Variables|Default|GetDash%20CD))
        (goto _label Reset)))))