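; Combat component that handles attack effects, currently only a stacking Hot buff triggered by Fire attacks.
; Each Fire hit adds stacks if the total stays within the default limit, then sets a looping timer that removes one stack per interval.
; Nothing stops that timer or floors the count at zero, and Tick prints the stack count for debugging.
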(event Custom|clearHotBuff
  ;[1 1 1] 攻击特效
  (Variables|Fire|SetHotBuffNumber (- (Variables|Fire|GetHotBuffNumber) 1)))

(event Custom|AttackEffect
  (params (AttackEffectType :type AttackEffectType%20Enum :default "NewEnumerator0"))
  ;[1 1 1] 攻击特效
  (switch Utilities|FlowControl|Switch|SwitchonAttackEffectType AttackEffectType
    (:NewEnumerator1
      (if (<= (+ (Variables|Fire|GetHotBuffNumber) (Variables|Fire|GetAddHotBuffNumber)) (Variables|Fire|GetDefaultHotBuffLimit))
        (Variables|Fire|SetHotBuffNumber (+ (Variables|Fire|GetHotBuffNumber) (Variables|Fire|GetAddHotBuffNumber))))
      (Utilities|Time|SetTimerbyEvent (delegate Custom|clearHotBuff) (Variables|Fire|GetHotBuffStillTime) true))))

(event EventTick
  (params (DeltaSeconds :type Float%20%28single-precision%29))
  (Development|PrintString (Utilities|String|ToString(Integer) (Variables|Fire|GetHotBuffNumber))))