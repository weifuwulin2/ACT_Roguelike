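; Damage component that rolls critical hits and applies damage to the stats of its own owner.
; CalculateDamage doubles damage when a random roll falls within the critical chance.
; GivingDamage casts the owner to BP_TopDownCharacter for player stats, falling back to Damageable for monster stats.
; IsShieldExist true routes to ChangeHealth and false to ChangeShieldValue, opposite to its name, and the ChangeHealth enum differs between player and monster.
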(event EventBeginPlay)

(event EventTick
  (params (DeltaSeconds :type Float%20%28single-precision%29)))

(fn GivingDamage
  (params (isShieldExist :type Boolean) (damage :type Float%20%28double-precision%29))
  (bind _returnvalue (Components|GetOwner))
  (bind _asbp_top_down_character (Utilities|Casting|CastToBP_TopDownCharacter _returnvalue)
    (:then
      (if isShieldExist
        (Default|ChangeHealth (Variables|/Game/Combat_XYH_WeiFu/Blueprints/BP_TopDownCharacter.BP_TopDownCharacter_C|GetBPC_PlayerStats _asbp_top_down_character) damage "NewEnumerator1")
        (else
          (Default|ChangeShieldValue (Variables|/Game/Combat_XYH_WeiFu/Blueprints/BP_TopDownCharacter.BP_TopDownCharacter_C|GetBPC_PlayerStats _asbp_top_down_character) damage "NewEnumerator1"))))
    (:CastFailed
      (bind _asdamageable (Utilities|Casting|CastToDamageable _returnvalue))
      (if isShieldExist
        (bind _monsterstats (Default|GetMonsterStats _asdamageable))
        (Default|ChangeHealth _monsterstats damage "NewEnumerator0")
        (else
          (Default|ChangeShieldValue _monsterstats damage "NewEnumerator1"))))))

(fn CalculateDamage
  (params (damage :type Float%20%28double-precision%29) (criticalChance :type Float%20%28double-precision%29))
  (LocalVariables|Setdmg damage)
  (if (> criticalChance 0.0)
    (if (<= (Math|Random|RandomFloatinRange 0.0 1.0) criticalChance)
      (LocalVariables|Setdmg (* damage 2.0))
      (else
        (LocalVariables|Setdmg damage))))
  (return (LocalVariables|Getdmg)))