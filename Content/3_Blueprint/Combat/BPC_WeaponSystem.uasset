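; Weapon component that switches the player's sword between its mounted and in-hand meshes and manages its fire look.
; BeginPlay caches the Niagara fire effect attached as the first child of the character's MountWeapon.
; OpenFireEffect applies the M_Sword04 material to both meshes and shows that effect.
; MountWeapon and HandWeapon events toggle mesh visibility, showing the effect only when mounted if BPCAttackEffect.CanFire is set, and hiding it in hand.
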(event Custom|MountWeapon
  ;[1 1 1] Weapon Idle
  (bind _asbp_top_down_character (Utilities|Casting|CastToBP_TopDownCharacter (Game|GetPlayerCharacter 0)))
  (Rendering|SetVisibility (Variables|/Game/Combat_XYH_WeiFu/Blueprints/BP_TopDownCharacter.BP_TopDownCharacter_C|GetHandWeapon _asbp_top_down_character) false false)
  (if (Variables|/Game/3_Blueprint/Combat/BPC_AttackEffect.BPC_AttackEffect_C|GetcanFire (Variables|/Game/Combat_XYH_WeiFu/Blueprints/BP_TopDownCharacter.BP_TopDownCharacter_C|GetBPC_AttackEffect _asbp_top_down_character))
    (Rendering|SetVisibility (Variables|Default|GetFireEffect_Mount) true false))
  (Rendering|SetVisibility (Variables|/Game/Combat_XYH_WeiFu/Blueprints/BP_TopDownCharacter.BP_TopDownCharacter_C|GetMountWeapon _asbp_top_down_character) true false))

(event Custom|HandWeapon
  ;[1 1 1] Weapon
  (bind _asbp_top_down_character (Utilities|Casting|CastToBP_TopDownCharacter (Game|GetPlayerCharacter 0)))
  (Rendering|SetVisibility (Variables|/Game/Combat_XYH_WeiFu/Blueprints/BP_TopDownCharacter.BP_TopDownCharacter_C|GetHandWeapon _asbp_top_down_character) true false)
  (Rendering|SetVisibility (Variables|/Game/Combat_XYH_WeiFu/Blueprints/BP_TopDownCharacter.BP_TopDownCharacter_C|GetMountWeapon _asbp_top_down_character) false false)
  (Rendering|SetVisibility (Variables|Default|GetFireEffect_Mount) false false))

(event Custom|OpenFireEffect
  ;[1 1 1] Fire VFX Init
  (bind _asbp_top_down_character (Utilities|Casting|CastToBP_TopDownCharacter (Game|GetPlayerCharacter 0)))
  (Rendering|Material|SetMaterial (Variables|/Game/Combat_XYH_WeiFu/Blueprints/BP_TopDownCharacter.BP_TopDownCharacter_C|GetHandWeapon _asbp_top_down_character) 0 "/Game/Sword_Fx/Materials/M_Sword04.M_Sword04")
  (Rendering|Material|SetMaterial (Variables|/Game/Combat_XYH_WeiFu/Blueprints/BP_TopDownCharacter.BP_TopDownCharacter_C|GetMountWeapon _asbp_top_down_character) 0 "/Game/Sword_Fx/Materials/M_Sword04.M_Sword04")
  (Rendering|SetVisibility (Variables|Default|GetFireEffect_Mount) true false))

(event EventBeginPlay
  ;[1 1 1] Event Start
  (bind _asbp_top_down_character (Utilities|Casting|CastToBP_TopDownCharacter (Game|GetPlayerCharacter 0)))
  (bind _asniagara_particle_system_component (Utilities|Casting|CastToNiagaraComponent (Components|GetChildComponent (Variables|/Game/Combat_XYH_WeiFu/Blueprints/BP_TopDownCharacter.BP_TopDownCharacter_C|GetMountWeapon _asbp_top_down_character) 0)))
  (Variables|Default|SetFireEffect_Mount _asniagara_particle_system_component))