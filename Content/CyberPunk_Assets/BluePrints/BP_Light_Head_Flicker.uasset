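; BP_Light_Head_Flicker is a light prop that, per its name, flickers, pairing a point light with a Sign mesh.
; The construction script creates a dynamic material instance on the sign's second material slot.
; On BeginPlay, a timeline's scaled LightIntensity curve sets the light intensity, while the material's Brightness is set to zero.
; A Delay using that same scaled value as its duration loops back to the intensity update.
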(event EventBeginPlay
  (bind _light_intensity (Timeline|Timeline_Intensity Play)
    (:Update
      (Rendering|Components|Light|SetIntensity (Variables|Default|GetPointLight) (* _light_intensity 6.76e+04) :!label _label)
      (Rendering|Material|SetScalarParameterValue (Variables|Default|GetDynamicMat) "Brightness" 0.0 :!class /Script/Engine.MaterialInstanceDynamic)
      (Utilities|FlowControl|Delay (* _light_intensity 6.76e+04))
      (goto _label))))

(fn ConstructionScript
  (bind _returnvalue (Rendering|Material|CreateDynamicMaterialInstance (Variables|Default|GetSign) 1 0 "None" :!class /Script/Engine.PrimitiveComponent))
  (Variables|Default|SetDynamicMat _returnvalue))