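; BP_Light_Florescent_Flicker is a fluorescent light whose brightness is animated by a timeline started on BeginPlay.
; The construction script creates a dynamic material from element 1 of the light's component.
; Timeline updates drive both point light intensity and material Brightness from the same scaled LightIntensity value.
; That value also sets a Delay, which loops back to reapply both.
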(event EventBeginPlay
  (bind _light_intensity (Timeline|Timeline_Intensity Play)
    (:Update
      (Rendering|Components|Light|SetIntensity (Variables|Default|GetPointLight) (* _light_intensity 75.0) :!label _label)
      (Rendering|Material|SetScalarParameterValue (Variables|Default|GetDynamicMat) "Brightness" (* _light_intensity 75.0) :!class /Script/Engine.MaterialInstanceDynamic)
      (Utilities|FlowControl|Delay (* _light_intensity 75.0))
      (goto _label))))

(fn ConstructionScript
  (bind _returnvalue (Rendering|Material|CreateDynamicMaterialInstance (Variables|Default|GetFlorecent%20light) 1 0 "None" :!class /Script/Engine.PrimitiveComponent))
  (Variables|Default|SetDynamicMat _returnvalue))