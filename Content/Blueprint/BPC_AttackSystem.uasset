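; Actor component that runs a four-hit melee attack combo for the top-down character.
; Attack input starts the step matching AttackIndex or buffers a press made mid-attack, which BasicAttackCombo uses to chain onward or reset via StopCombo.
; DoOnce-gated attack events play montages after a short delay and advance the index.
; Attack speed bonus scales playback for all but the final hit.
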(event Custom|BasicAttack
  ;[1 1 1] basic attack
  (if (Variables|Default|GetisAttacking)
    (Variables|Default|SetsaveAttack true)
    (else
      (Variables|Default|SetisAttacking true)
      (switch int (Variables|Default|GetattackIndex)
        (:0
          (CallFunction|Attack1))
        (:1
          (CallFunction|Attack2))
        (:2
          (CallFunction|Attack3))
        (:3
          (CallFunction|Attack4))))))

(event Custom|BasicAttackCombo
  ;[1 1 1] Combo continue
  (if (Variables|Default|GetsaveAttack)
    (Variables|Default|SetsaveAttack false)
    (switch int (Variables|Default|GetattackIndex)
      (:0
        (CallFunction|Attack1))
      (:1
        (CallFunction|Attack2))
      (:2
        (CallFunction|Attack3))
      (:3
        (CallFunction|Attack4)))
    (else
      (CallFunction|StopCombo))))

(event Custom|Attack_2
  ;[1 1 1] Attack_2
  (Utilities|FlowControl|DoOnce false :!label _label
    (:Completed
      (Utilities|FlowControl|Delay 0.1)
      (Animation|Montage|PlayMontage (Variables|Default|GetCharacterMesh) "/Game/Animations/Character/Combat/StandingMeleeAttackDownward_1__UE_2_Montage.StandingMeleeAttackDownward_1__UE_2_Montage" (* (Variables|Default|GetstartingAttackSpeed) (+ 1.0 (Variables|Default|GetcurrentAttackSpeed)))
        (:then
          (Variables|Default|SetattackIndex 2)
          (goto _label Reset))))))

(event Custom|Attack_3
  ;[1 1 1] Attack_3
  (Utilities|FlowControl|DoOnce false :!label _label
    (:Completed
      (Utilities|FlowControl|Delay 0.1)
      (Animation|Montage|PlayMontage (Variables|Default|GetCharacterMesh) "/Game/Animations/Character/Combat/StandingMeleeAttackBackhand_UE_3_Montage.StandingMeleeAttackBackhand_UE_3_Montage" (* (Variables|Default|GetstartingAttackSpeed) (+ 1.0 (Variables|Default|GetcurrentAttackSpeed)))
        (:then
          (Variables|Default|SetattackIndex 3)
          (goto _label Reset))))))

(event Custom|StopCombo
  ;[1 1 1] Stop the whole combo/attack
  (Variables|Default|SetisAttacking false)
  (Variables|Default|SetattackIndex 0))

(event Custom|Attack_4
  ;[1 1 1] Attack_4
  (Utilities|FlowControl|DoOnce false :!label _label
    (:Completed
      (Utilities|FlowControl|Delay 0.1)
      (Animation|Montage|PlayMontage (Variables|Default|GetCharacterMesh) "/Game/Animations/Character/Combat/StandingMeleeAttack360Low_1__UE_4_Montage.StandingMeleeAttack360Low_1__UE_4_Montage" (Variables|Default|GetstartingAttackSpeed)
        (:then
          (Variables|Default|SetattackIndex 4)
          (goto _label Reset))))))

(event Custom|Attack_1
  ;[1 1 1] Attack_1
  (Utilities|FlowControl|DoOnce false :!label _label
    (:Completed
      (Utilities|FlowControl|Delay 0.1)
      (Animation|Montage|PlayMontage (Variables|Default|GetCharacterMesh) "/Game/Animations/Character/Combat/StandingMeleeAttackHorizontal_2__UE_1_Montage.StandingMeleeAttackHorizontal_2__UE_1_Montage" (* (Variables|Default|GetstartingAttackSpeed) (+ 1.0 (Variables|Default|GetcurrentAttackSpeed)))
        (:then
          (Variables|Default|SetattackIndex 1)
          (goto _label Reset))))))

(event Input|EnhancedActionEvents|EnhancedInputActionIA_Attack
  (params (ActionValue :type Boolean) (ElapsedSeconds :type Float%20%28double-precision%29) (TriggeredSeconds :type Float%20%28double-precision%29) (InputAction :type Input%20Action%20Object%20Reference :default "/Game/TopDown/Input/Actions/IA_Attack.IA_Attack"))
  ;[1 1 1] Input and attack
  (:Triggered
    (if (Variables|Default|GetcanAttack)
      (CallFunction|BasicAttack))))

(event EventBeginPlay
  ;[1 1 1] Set the character at start
  (bind _asbp_top_down_character (Utilities|Casting|CastToBP_TopDownCharacter (Components|GetOwner)))
  (Variables|Default|SetCharacterMesh (Variables|/Script/Engine.Character|GetMesh _asbp_top_down_character)))