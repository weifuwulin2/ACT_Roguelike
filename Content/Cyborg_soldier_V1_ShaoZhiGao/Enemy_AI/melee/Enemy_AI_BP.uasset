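; Melee enemy character that sets up its health-bar widget and alive Blackboard flag on BeginPlay, turning the bar toward the camera once.
; GetHit checks the MonsterStats component's health, playing a DoOnce-gated hit montage followed by a launch along the player's forward vector, or calling Death.
; Death disables movement and collision, plays a knockdown, detaches the controller and destroys the actor after a delay.
; Getters expose stats, damage-calculation, widget and monster key.
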(event Custom|Hurt
  ;[1 1 1] 受到伤害的相关判断
  (Utilities|FlowControl|Sequence
    (:then_0
      (if (> (Variables|/Game/3_Blueprint/MonsterStats/BPC_MonsterStats.BPC_MonsterStats_C|GetCurrentHealth (Variables|Default|GetBPC_MonsterStats)) 0.0)
        (Utilities|FlowControl|DoOnce false :!label _label
          (:Completed
            (Animation|Montage|PlayMontage (Variables|Character|GetMesh) "/Game/Cyborg_soldier_V1_ShaoZhiGao/Enemy_Animation/melee_montage/Frank_RPG_Assassin_Hit_Knockback_IP_Montage.Frank_RPG_Assassin_Hit_Knockback_IP_Montage" 1.5 0.3
              (:OnCompleted
                (bind _asbp_top_down_character (Utilities|Casting|CastToBP_TopDownCharacter (Game|GetPlayerCharacter 0)))
                (Transformation|SetActorRotation (Math|Rotator|FindLookatRotation (Math|Vector|GetForwardVector (Transformation|GetActorRotation _asbp_top_down_character)) (Transformation|GetActorForwardVector self)))
                (Character|LaunchCharacter (* (Math|Vector|GetForwardVector (Transformation|GetActorRotation _asbp_top_down_character)) 5e+01) false false)
                (goto _label Reset)))))
        (else
          (CallFunction|Death))))
    (:then_1
      (Development|PrintString (Utilities|String|ToString(Float) (Variables|/Game/3_Blueprint/MonsterStats/BPC_MonsterStats.BPC_MonsterStats_C|GetCurrentHealth (Variables|Default|GetBPC_MonsterStats)))))))

(event Custom|Death
  ;[1 1 1] 死亡
  (Pawn|Components|CharacterMovement|DisableMovement (Variables|Character|GetCharacterMovement))
  (Collision|SetCollisionEnabled (Variables|Character|GetMesh) "NoCollision")
  (Animation|Montage|PlayMontage (Variables|Character|GetMesh) "/Game/Cyborg_soldier_V1_ShaoZhiGao/Enemy_Animation/melee_montage/Frank_RPG_Assassin_Hit_Knockdown_IP_Montage.Frank_RPG_Assassin_Hit_Knockdown_IP_Montage"
    (:then
      (Class|Pawn|DetachfromControllerPendingDestroy)
      (Development|PrintString "death")
      (Rendering|SetVisibility (Variables|Default|Gethealthy) false false)
      (Utilities|FlowControl|Delay 1.0)
      (Actor|DestroyActor))))

(event Custom|旋转血条
  (bind _healthy (Variables|Default|Gethealthy))
  ;[1 1 1] 血条转向摄像机
  (Transformation|SetWorldRotation _healthy (Math|Rotator|FindLookatRotation (Transformation|GetWorldLocation _healthy) (Camera|GetCameraLocation (Game|GetPlayerCameraManager 0))) false false))

(event EventTick
  (params (DeltaSeconds :type Float%20%28single-precision%29))
  ;[1 1 1] 弃用
)

(event EventBeginPlay
  ;[1 1 1] 设定血量
  (CallFunction|旋转血条)
  (bind _asai_blood (Utilities|Casting|CastToAI_Blood (UserInterface|GetUserWidgetObject (Variables|Default|Gethealthy))))
  (bind _output_get (Variables|Default|SetAs%20AI%20Blood _asai_blood))
  (Variables|/Game/Cyborg_soldier_V1_ShaoZhiGao/Enemy_AI/AI/AI_Blood.AI_Blood_C|Sethealthy _output_get 5e+01)
  (bind _output_get_2 (Variables|Default|Set存活 true))
  (AI|Components|Blackboard|SetValueasBool (AI|GetBlackboard 0) (Utilities|Name|MakeLiteralName "活着？") _output_get_2))

(event EventGetHit
  ;[1 1 1] 受到伤害的相关判断
  (CallFunction|Hurt))

(fn ConstructionScript)

(fn ReturnDMGCalculation
  (return (Variables|Default|GetBPC_DamageCalculation)))

(fn GetDamageCalcuationBPC
  (return (Variables|Default|GetBPC_DamageCalculation)))

(fn GetHUD
  (return (Variables|Default|Gethealthy)))

(fn GetMonsterKey
  (return (Variables|Default|GetMonsterKey)))

(fn GetMonsterStats
  (return (Variables|Default|GetBPC_MonsterStats)))