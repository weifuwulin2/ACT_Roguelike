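; Pickup handgun weapon Blueprint for the cyborg soldier, extending a parent weapon with cosmetic attachment, magazine and effect logic.
; Events show or hide three magazine parts by swapping material slots with an invisible material, with the default set chosen by AutoReload.
; Muzzle smoke requires ammo and shifts forward with a silencer, and an attached scope hides its slot cover.
; Tick updates the laser point only while this is the current weapon with a visible flashlight.
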(event EventScopeAttached
  ;[1 1 1] Scope Attached
  (CallFunction|SetScopeSlotCoverVisibility))

(event EventMag01InvisEvnt
  ;[1 1 1] Mag Visibility
  (Rendering|Material|SetMaterial (Variables|Default|GetWeapon_SKMesh) 2 "/Game/Cyborg_soldier_V1_ShaoZhiGao/cgHandgun/Weapons/Materials/MasterMaterials/MM_Invisible.MM_Invisible"))

(event EventMag02VisEvnt
  ;[1 1 1] Mag Visibility
  (Rendering|Material|SetMaterial (Variables|Default|GetWeapon_SKMesh) 4 "/Game/Cyborg_soldier_V1_ShaoZhiGao/cgHandgun/Weapons/Materials/MaterialInstances/MI_GunColorVariations/MI_cgHg_Lower_Headshot.MI_cgHg_Lower_Headshot"))

(event EventMag02InvisEvnt
  ;[1 1 1] Mag Visibility
  (Rendering|Material|SetMaterial (Variables|Default|GetWeapon_SKMesh) 4 "/Game/Cyborg_soldier_V1_ShaoZhiGao/cgHandgun/Weapons/Materials/MasterMaterials/MM_Invisible.MM_Invisible"))

(event EventMagVisible
  (bind _weapon_skmesh (Variables|Default|GetWeapon_SKMesh))
  ;[0 0 0] Mag Visible
  (if (Variables|Default|GetAutoReload?)
    ;;[1 1 1] Mag_Empty
    (Rendering|Material|SetMaterial _weapon_skmesh 3 "/Game/Cyborg_soldier_V1_ShaoZhiGao/cgHandgun/Weapons/Materials/MaterialInstances/MI_GunColorVariations/MI_cgHg_Lower_Headshot.MI_cgHg_Lower_Headshot")
    ;;[1 1 1] Mag_01
    (Rendering|Material|SetMaterial _weapon_skmesh 2 "/Game/Cyborg_soldier_V1_ShaoZhiGao/cgHandgun/Weapons/Materials/MasterMaterials/MM_Invisible.MM_Invisible")
    ;;[1 1 1] Mag_02
    (Rendering|Material|SetMaterial _weapon_skmesh 4 "/Game/Cyborg_soldier_V1_ShaoZhiGao/cgHandgun/Weapons/Materials/MasterMaterials/MM_Invisible.MM_Invisible")
    (else
      (Rendering|Material|SetMaterial _weapon_skmesh 3 "/Game/Cyborg_soldier_V1_ShaoZhiGao/cgHandgun/Weapons/Materials/MasterMaterials/MM_Invisible.MM_Invisible")
      (Rendering|Material|SetMaterial _weapon_skmesh 2 "/Game/Cyborg_soldier_V1_ShaoZhiGao/cgHandgun/Weapons/Materials/MaterialInstances/MI_GunColorVariations/MI_cgHg_Lower_Headshot.MI_cgHg_Lower_Headshot")
      (Rendering|Material|SetMaterial _weapon_skmesh 4 "/Game/Cyborg_soldier_V1_ShaoZhiGao/cgHandgun/Weapons/Materials/MasterMaterials/MM_Invisible.MM_Invisible"))))

(event EventMagEmptyVisEvnt
  ;[1 1 1] Mag Visibility
  (Rendering|Material|SetMaterial (Variables|Default|GetWeapon_SKMesh) 3 "/Game/Cyborg_soldier_V1_ShaoZhiGao/cgHandgun/Weapons/Materials/MaterialInstances/MI_GunColorVariations/MI_cgHg_Lower_Headshot.MI_cgHg_Lower_Headshot"))

(event EventMagEmptyInvisEvnt
  ;[1 1 1] Mag Visibility
  (Rendering|Material|SetMaterial (Variables|Default|GetWeapon_SKMesh) 3 "/Game/Cyborg_soldier_V1_ShaoZhiGao/cgHandgun/Weapons/Materials/MasterMaterials/MM_Invisible.MM_Invisible"))

(event EventBSmokeStop
  ;[1 1 1] MuzzleSmoke
  (Components|Activation|Deactivate (Variables|Default|GetMuzzleSmoke_PS))
  (Transformation|SetRelativeLocation (Variables|Default|GetMuzzleSmoke_PS) "0, 0, 0" false false))

(event EventBSmokeStart
  ;[1 1 1] MuzzleSmoke
  (if (> (.AmmoCurrent (Utilities|Struct|BreakBP_WeaponData_Struct (Variables|Default|GetWeaponData))) 0)
    (Utilities|FlowControl|Sequence
      (:then_0
        _)
      (:then_1
        (goto _label Reset)))
    (else
      (Utilities|FlowControl|DoOnce false :!label _label
        (:Completed
          _))))
  (Components|Activation|Activate (Variables|Default|GetMuzzleSmoke_PS) false)
  (if (Rendering|IsVisible (Variables|Default|GetSM_Silencer))
    (Transformation|SetRelativeLocation (Variables|Default|GetMuzzleSmoke_PS) (+ (Variables|/Script/Engine.SceneComponent|GetRelativeLocation (Variables|Default|GetMuzzleSmoke_PS)) "20.000000, 0, 0") false false)
    (else
      (Transformation|SetRelativeLocation (Variables|Default|GetMuzzleSmoke_PS) "0, 0, 0" false false))))

(event EventMag01VisEvnt
  ;[1 1 1] Mag Visibility
  (Rendering|Material|SetMaterial (Variables|Default|GetWeapon_SKMesh) 2 "/Game/Cyborg_soldier_V1_ShaoZhiGao/cgHandgun/Weapons/Materials/MaterialInstances/MI_GunColorVariations/MI_cgHg_Lower_Headshot.MI_cgHg_Lower_Headshot"))

(event EventTick
  (params (DeltaSeconds :type Float%20%28single-precision%29))
  ;[1 1 1] Laser
  (if (not (and (== self (Variables|/Game/Cyborg_soldier_V1_ShaoZhiGao/cgHandgun/FPS_Arms/Bluprints/BP_FPS_Arms.BP_FPS_Arms_C|GetCurrentWeapon (Variables|Default|GetCharacter%20Ref))) (Rendering|IsVisible (Variables|Default|GetSM_Flashlight))))
    (Rendering|SetVisibility (Variables|Default|GetSM_Laser) false false)
    (Rendering|SetVisibility (Variables|Default|GetLaser_Point) false false)
    (else
      (CallFunction|LaserPointPosition))))

(fn ConstructionScript
  (|CallParentFunction))

(fn SetScopeSlotCoverVisibility
  (bind _scope_slot_cover (Variables|Default|GetScope%20Slot%20Cover))
  (if (Rendering|IsVisible (Variables|Default|GetSM_Scope))
    (Rendering|SetVisibility _scope_slot_cover false false)
    (else
      (Rendering|SetVisibility _scope_slot_cover true false)))
  (return))