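; BP_cgHg_Auto is a pickup handgun Blueprint that adds weapon-specific cosmetic behavior to its parent gun class.
; Events toggle three magazine meshes and reattach the empty one between sockets for reload montages, with initial visibility set by AutoReload.
; Muzzle smoke depends on remaining ammo and shifts forward for a visible silencer, while a scope hides its slot cover.
; Tick updates the laser point only when this is the current weapon and the flashlight mesh is visible.
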(event EventScopeAttached
  ;[1 1 1] Scope Attached
  (CallFunction|SetScopeSlotCoverVisibility))

(event EventMag01InvisEvnt
  ;[1 1 1] Mag Visibility
  (Rendering|SetVisibility (Variables|Default|GetMagazine_01) false false))

(event EventMag02VisEvnt
  ;[1 1 1] Mag Visibility
  (Rendering|SetVisibility (Variables|Default|GetMagazine_02) true false))

(event EventMag02InvisEvnt
  ;[1 1 1] Mag Visibility
  (Rendering|SetVisibility (Variables|Default|GetMagazine_02) false false))

(event EventMagVisible
  (bind _magazine_01 (Variables|Default|GetMagazine_01))
  (bind _magazine_02 (Variables|Default|GetMagazine_02))
  (bind _magazine_empty (Variables|Default|GetMagazine_Empty))
  ;[1 1 1] Mag Visible
  (if (Variables|Default|GetAutoReload?)
    (Rendering|SetVisibility _magazine_empty true false)
    (Rendering|SetVisibility _magazine_01 false false)
    (Rendering|SetVisibility _magazine_02 false false)
    (else
      (Rendering|SetVisibility _magazine_empty false false)
      (Rendering|SetVisibility _magazine_01 true false)
      (Rendering|SetVisibility _magazine_02 false false))))

(event EventMagDetachEvnt
  ;[1 1 1] Attach MagEmpty to Mag 01 socket.       Need in      "cgHandgun_FullReload_Montage_Fast"
  (Transformation|AttachComponentToComponent (Variables|Default|GetMagazine_Empty) (Variables|Default|GetWeapon_SKMesh) "MSocket_00" "SnapToTarget" "SnapToTarget" "SnapToTarget" true))

(event EventMagAttachEvnt
  ;[1 1 1] Attach MagEmpty to Mag 01 socket.       Need in      "cgHandgun_FullReload_Montage_Fast"
  (Transformation|AttachComponentToComponent (Variables|Default|GetMagazine_Empty) (Variables|Default|GetWeapon_SKMesh) "MSocket_01" "SnapToTarget" "SnapToTarget" "SnapToTarget" true))

(event EventMagEmptyVisEvnt
  ;[1 1 1] Mag Visibility
  (Rendering|SetVisibility (Variables|Default|GetMagazine_Empty) true false))

(event EventMagEmptyInvisEvnt
  ;[1 1 1] Mag Visibility
  (Rendering|SetVisibility (Variables|Default|GetMagazine_Empty) false false))

(event EventBSmokeStop
  ;[1 1 1] MuzzleSmoke
  (Components|Activation|Deactivate (Variables|Default|GetMuzzleSmoke_PS))
  (Transformation|SetRelativeLocation (Variables|Default|GetMuzzleSmoke_PS) "0, 0, 0" false false))

(event EventBSmokeStart
  ;[1 1 1] MuzzleSmoke
  (if (> (.AmmoCurrent (Utilities|Struct|BreakBP_WeaponData_Struct (Variables|Default|GetWeaponData))) 0)
    (Utilities|FlowControl|Sequence
      (:then_0
        _)
      (:then_1
        (goto _label Reset)))
    (else
      (Utilities|FlowControl|DoOnce false :!label _label
        (:Completed
          _))))
  (Components|Activation|Activate (Variables|Default|GetMuzzleSmoke_PS) false)
  (if (Rendering|IsVisible (Variables|Default|GetSM_Silencer))
    (Transformation|SetRelativeLocation (Variables|Default|GetMuzzleSmoke_PS) (+ (Variables|/Script/Engine.SceneComponent|GetRelativeLocation (Variables|Default|GetMuzzleSmoke_PS)) "20.000000, 0, 0") false false)
    (else
      (Transformation|SetRelativeLocation (Variables|Default|GetMuzzleSmoke_PS) "0, 0, 0" false false))))

(event EventMag01VisEvnt
  ;[1 1 1] Mag Visibility
  (Rendering|SetVisibility (Variables|Default|GetMagazine_01) true false))

(event EventTick
  (params (DeltaSeconds :type Float%20%28single-precision%29))
  ;[1 1 1] Laser
  (if (not (and (== self (Variables|/Game/Cyborg_soldier_V1_ShaoZhiGao/cgHandgun/FPS_Arms/Bluprints/BP_FPS_Arms.BP_FPS_Arms_C|GetCurrentWeapon (Variables|Default|GetCharacter%20Ref))) (Rendering|IsVisible (Variables|Default|GetSM_Flashlight))))
    (Rendering|SetVisibility (Variables|Default|GetSM_Laser) false false)
    (Rendering|SetVisibility (Variables|Default|GetLaser_Point) false false)
    (else
      (CallFunction|LaserPointPosition))))

(fn ConstructionScript
  (|CallParentFunction))

(fn SetScopeSlotCoverVisibility
  (bind _scope_slot_cover (Variables|Default|GetScope%20Slot%20Cover))
  (if (Rendering|IsVisible (Variables|Default|GetSM_Scope))
    (Rendering|SetVisibility _scope_slot_cover false false)
    (else
      (Rendering|SetVisibility _scope_slot_cover true false)))
  (return))