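; An interactable handgun ammo pickup that refills the reserve ammo of the player's current weapon.
; On interaction it accepts four handgun variants by weapon name, reads that weapon's ammo pool, and prints a message if ammo is full or mismatched.
; Otherwise it plays pickup sounds, sets AmmoMax through a cap check that any non-negative reserve passes, so it jumps to the pool value, destroys itself and auto-reloads an empty magazine.
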(event EventBeginPlay
  (|CallParentFunction) ; This node is disabled and will not be called.\nDrag off pins to build functionality.
)

(event Collision|EventActorBeginOverlap
  (params (OtherActor :type Actor%20Object%20Reference))
  (|CallParentFunction OtherActor) ; This node is disabled and will not be called.\nDrag off pins to build functionality.
)

(event EventTick
  (params (DeltaSeconds :type Float%20%28single-precision%29))
  (|CallParentFunction DeltaSeconds) ; This node is disabled and will not be called.\nDrag off pins to build functionality.
)

(event EventOnInteracted
  (params (Player%200 :type BP%20FPS%20Arms%20Object%20Reference))
  (bind _pickupammo (Variables|Default|GetPickUpAmmo))
  (bind _currentweapon (Variables|/Game/Cyborg_soldier_V1_ShaoZhiGao/cgHandgun/FPS_Arms/Bluprints/BP_FPS_Arms.BP_FPS_Arms_C|GetCurrentWeapon Player%200))
  (bind _currentweapon_2 (Variables|/Game/Cyborg_soldier_V1_ShaoZhiGao/cgHandgun/FPS_Arms/Bluprints/BP_FPS_Arms.BP_FPS_Arms_C|GetCurrentWeapon Player%200))
  (bind _weapondata (Variables|/Game/Cyborg_soldier_V1_ShaoZhiGao/cgHandgun/Weapons/Blueprints/PickUp_Master/Gun/BP_Weapon_Base.BP_Weapon_Base_C|GetWeaponData _currentweapon_2))
  (bind _weapondata_2 (Variables|/Game/Cyborg_soldier_V1_ShaoZhiGao/cgHandgun/Weapons/Blueprints/PickUp_Master/Gun/BP_Weapon_Base.BP_Weapon_Base_C|GetWeaponData _currentweapon))
  (bind _ammomax (Utilities|Struct|BreakBP_WeaponData_Struct _weapondata_2))
  (bind _returnvalue (+ _pickupammo _ammomax))
  (Utilities|IsValid _currentweapon
    (:Is%20Valid
      (Variables|Default|SetPickupAmmo (Variables|/Game/Cyborg_soldier_V1_ShaoZhiGao/cgHandgun/Weapons/Blueprints/PickUp_Master/Gun/BP_Weapon_Base.BP_Weapon_Base_C|GetCG_Handgun_AMMOPool _currentweapon))
      (if (CallFunction|CGHundguns _currentweapon)
        (if (== _ammomax (Variables|Default|GetPickUpAmmo))
          (Development|PrintString "Full Ammo" true true "(R=0.000000,G=0.200000,B=1.000000,A=1.000000)")
          (else
            (CallFunction|PickUpSound Player%200)
            (CallFunction|AmmoPickUpSound Player%200)
            (if (>= _returnvalue (Variables|Default|GetPickUpAmmo))
              (Utilities|Struct|SetmembersinBP_WeaponData_Struct _weapondata (Variables|Default|GetPickUpAmmo))
              (Actor|DestroyActor)
              (if (== (.AmmoCurrent (Utilities|Struct|BreakBP_WeaponData_Struct _weapondata)) 0)
                (Default|AutoReload _currentweapon_2))
              (else
                (Utilities|Struct|SetmembersinBP_WeaponData_Struct _weapondata _returnvalue)
                (Actor|DestroyActor)))))
        (else
          (Development|PrintString "Ammo Not Match" true true "(R=1.000000,G=0.000000,B=0.000000,A=1.000000)"))))))

(fn ConstructionScript
  (|CallParentFunction))

(fn CGHundguns
  (params (Name :type BP%20Weapon%20Base%20Object%20Reference))
  (bind _weaponname (Variables|/Game/Cyborg_soldier_V1_ShaoZhiGao/cgHandgun/Weapons/Blueprints/PickUp_Master/Gun/BP_Weapon_Base.BP_Weapon_Base_C|GetWeaponName Name))
  (return (Math|Boolean|ORBoolean (Utilities|Name|Equal(Name) _weaponname "CG_Handgun") (Utilities|Name|Equal(Name) _weaponname "CG_Hg_Auto") (Utilities|Name|Equal(Name) _weaponname "CG_Hg_ToggleAuto") (Utilities|Name|Equal(Name) _weaponname "CG_Hg_comb"))))

(fn AmmoPickUpSound
  (params (Out_Player :type BP%20FPS%20Arms%20Object%20Reference))
  (Audio|PlaySoundatLocation "/Game/Cyborg_soldier_V1_ShaoZhiGao/cgHandgun/Weapons/Audio/SC_Mag_insert_Empty_Cue.SC_Mag_insert_Empty_Cue" (Transformation|GetWorldLocation (Variables|/Game/Cyborg_soldier_V1_ShaoZhiGao/cgHandgun/FPS_Arms/Bluprints/BP_FPS_Arms.BP_FPS_Arms_C|GetArms Out_Player)) "0, 0, 0" 1.0 1.0 0.0 0 0 0 0)
  (return))