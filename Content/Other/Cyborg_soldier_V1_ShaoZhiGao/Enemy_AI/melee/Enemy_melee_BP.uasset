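; Melee enemy AI character with a health widget, hit reactions and a death sequence, driven through Blackboard flags for alive and hurt.
; AnyDamage only raises the hurt flag; the separate Hurt event subtracts health behind a DoOnce, then plays a random hit montage or clears alive.
; Death disables movement and collision, plays a knockdown, detaches the controller and destroys the actor.
; The health bar faces the camera only at BeginPlay; Tick prints debug health.
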(event Custom|Hurt
  (bind _as_ai_blood (Variables|Default|GetAs%20AI%20Blood))
  ;[1 1 1] 受到伤害的相关判断
  (Utilities|FlowControl|DoOnce false :!label _label
    (:Completed
      (bind _output_get (Variables|/Game/Other/Cyborg_soldier_V1_ShaoZhiGao/Enemy_AI/melee/melee_AI/AI_Blood.AI_Blood_C|Sethealthy _as_ai_blood (- (Variables|/Game/Other/Cyborg_soldier_V1_ShaoZhiGao/Enemy_AI/melee/melee_AI/AI_Blood.AI_Blood_C|Gethealthy _as_ai_blood) (stale Game|Damage|EventAnyDamage Damage))))
      (if (> _output_get 0.0)
        (Animation|Montage|PlayMontage (Variables|Character|GetMesh) (.OutItem (Utilities|Array|Random (Utilities|Array|MakeArray "/Game/Other/Cyborg_soldier_V1_ShaoZhiGao/Enemy_Animation/melee_montage/Frank_RPG_Assassin_Hit02_Montage.Frank_RPG_Assassin_Hit02_Montage" "/Game/Other/Cyborg_soldier_V1_ShaoZhiGao/Enemy_Animation/melee_montage/Frank_RPG_Assassin_Hit03_Montage.Frank_RPG_Assassin_Hit03_Montage" "/Game/Other/Cyborg_soldier_V1_ShaoZhiGao/Enemy_Animation/melee_montage/Frank_RPG_Assassin_Hit_Knockback_IP_Montage.Frank_RPG_Assassin_Hit_Knockback_IP_Montage")))
          (:OnCompleted
            (bind _output_get_2 (Variables|Default|Set受伤 false))
            (AI|Components|Blackboard|SetValueasBool (AI|GetBlackboard 0) (Utilities|Name|MakeLiteralName "受到伤害？") _output_get_2)
            (goto _label Reset)))
        (else
          (bind _output_get_3 (Variables|Default|Set存活 false))
          (AI|Components|Blackboard|SetValueasBool (AI|GetBlackboard 0) (Utilities|Name|MakeLiteralName "活着？") _output_get_3))))))

(event Custom|Death
  ;[1 1 1] 死亡
  (Pawn|Components|CharacterMovement|DisableMovement (Variables|Character|GetCharacterMovement))
  (Collision|SetCollisionEnabled (Variables|Character|GetMesh) "NoCollision")
  (Animation|Montage|PlayMontage (Variables|Character|GetMesh) "/Game/Other/Cyborg_soldier_V1_ShaoZhiGao/Enemy_Animation/melee_montage/Frank_RPG_Assassin_Hit_Knockdown_IP_Montage.Frank_RPG_Assassin_Hit_Knockdown_IP_Montage"
    (:then
      (Class|Pawn|DetachfromControllerPendingDestroy)
      (Rendering|SetVisibility (Variables|Default|Gethealthy) false false)
      (Utilities|FlowControl|Delay 1.0)
      (Actor|DestroyActor))))

(event Custom|旋转血条
  (bind _healthy (Variables|Default|Gethealthy))
  ;[1 1 1] 血条转向摄像机
  (Transformation|SetWorldRotation _healthy (Math|Rotator|FindLookatRotation (Transformation|GetWorldLocation _healthy) (Camera|GetCameraLocation (Game|GetPlayerCameraManager 0))) false false))

(event Game|Damage|EventAnyDamage
  (params (Damage :type Float%20%28single-precision%29) (DamageType :type Damage%20Type%20Object%20Reference) (InstigatedBy :type Controller%20Object%20Reference) (DamageCauser :type Actor%20Object%20Reference))
  ;[1 1 1] 受到伤害的相关判断
  (bind _output_get (Variables|Default|Set受伤 true))
  (AI|Components|Blackboard|SetValueasBool (AI|GetBlackboard 0) (Utilities|Name|MakeLiteralName "受到伤害？") _output_get))

(event EventTick
  (params (DeltaSeconds :type Float%20%28single-precision%29))
  ;[1 1 1] 弃用
  (Development|PrintString (Utilities|String|ToString(Float) (Variables|/Game/Other/Cyborg_soldier_V1_ShaoZhiGao/Enemy_AI/melee/melee_AI/AI_Blood.AI_Blood_C|Gethealthy (Variables|Default|GetAs%20AI%20Blood)))))

(event EventBeginPlay
  ;[1 1 1] 设定血量
  (CallFunction|旋转血条)
  (bind _asai_blood (Utilities|Casting|CastToAI_Blood (UserInterface|GetUserWidgetObject (Variables|Default|Gethealthy))))
  (bind _output_get (Variables|Default|SetAs%20AI%20Blood _asai_blood))
  (Variables|/Game/Other/Cyborg_soldier_V1_ShaoZhiGao/Enemy_AI/melee/melee_AI/AI_Blood.AI_Blood_C|Sethealthy _output_get 5e+01)
  (bind _output_get_2 (Variables|Default|Set存活 true))
  (AI|Components|Blackboard|SetValueasBool (AI|GetBlackboard 0) (Utilities|Name|MakeLiteralName "活着？") _output_get_2))

(fn ConstructionScript)