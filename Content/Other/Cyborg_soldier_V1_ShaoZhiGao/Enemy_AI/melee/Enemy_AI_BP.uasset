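; Melee enemy character that handles hit reactions, death and sword damage against the top-down player.
; BeginPlay initializes the health widget and the blackboard alive flag.
; Hurt checks the monster stats component, playing a knockback montage with launch, or detaching the controller and destroying the actor on death.
; A looping timer drives gated sphere traces along the blade that damage the player; getters expose components, with range, patrol and speed functions stubbed.
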(event Custom|Hurt
  ;[1 1 1] 受到伤害的相关判断
  (Utilities|FlowControl|Sequence
    (:then_0
      (if (> (Variables|/Game/3_Blueprint/MonsterStats/BPC_MonsterStats.BPC_MonsterStats_C|GetCurrentHealth (Variables|Default|GetBPC_MonsterStats)) 0.0)
        (Utilities|FlowControl|DoOnce false :!label _label
          (:Completed
            (Animation|Montage|PlayMontage (Variables|Character|GetMesh) "/Game/Other/Cyborg_soldier_V1_ShaoZhiGao/Enemy_Animation/melee_montage/Frank_RPG_Assassin_Hit_Knockback_IP_Montage.Frank_RPG_Assassin_Hit_Knockback_IP_Montage" 1.5 0.3
              (:OnCompleted
                (bind _asbp_top_down_character (Utilities|Casting|CastToBP_TopDownCharacter (Game|GetPlayerCharacter 0)))
                (Transformation|SetActorRotation (Math|Rotator|FindLookatRotation (Math|Vector|GetForwardVector (Transformation|GetActorRotation _asbp_top_down_character)) (Transformation|GetActorForwardVector self)))
                (Character|LaunchCharacter (* (Math|Vector|GetForwardVector (Transformation|GetActorRotation _asbp_top_down_character)) 5e+01) false false)
                (goto _label Reset)))))
        (else
          (CallFunction|Death))))
    (:then_1
      (Development|PrintString (Utilities|String|ToString(Float) (Variables|/Game/3_Blueprint/MonsterStats/BPC_MonsterStats.BPC_MonsterStats_C|GetCurrentHealth (Variables|Default|GetBPC_MonsterStats)))))))

(event Custom|Death
  ;[1 1 1] 死亡
  (Utilities|FlowControl|DoOnce false
    (:Completed
      (Pawn|Components|CharacterMovement|DisableMovement (Variables|Character|GetCharacterMovement))
      (Collision|SetCollisionEnabled (Variables|Character|GetMesh) "NoCollision")
      (Animation|Montage|PlayMontage (Variables|Character|GetMesh) "/Game/Other/Cyborg_soldier_V1_ShaoZhiGao/Enemy_Animation/melee_montage/Frank_RPG_Assassin_Hit_Knockdown_IP_Montage.Frank_RPG_Assassin_Hit_Knockdown_IP_Montage"
        (:then
          (Class|Pawn|DetachfromControllerPendingDestroy)
          (Development|PrintString "death")
          (Rendering|SetVisibility (Variables|Default|Gethealthy) false false)
          (Utilities|FlowControl|Delay 1.0)
          (Actor|DestroyActor))))))

(event Custom|旋转血条
  (bind _healthy (Variables|Default|Gethealthy))
  ;[1 1 1] 血条转向摄像机
  (Transformation|SetWorldRotation _healthy (Math|Rotator|FindLookatRotation (Transformation|GetWorldLocation _healthy) (Camera|GetCameraLocation (Game|GetPlayerCameraManager 0))) false false))

(event EventChangeHealth
  (params (MonsterStats :type BPC%20Monster%20Stats%20Object%20Reference) (Damage :type Float%20%28double-precision%29) (IncreaseType :type IncreaseEnum%20Enum :default "NewEnumerator0")))

(event EventTick
  (params (DeltaSeconds :type Float%20%28single-precision%29))
  ;[1 1 1] 弃用
)

(event EventBeginPlay
  ;[1 1 1] 设定血量
  (CallFunction|旋转血条)
  (bind _asai_blood (Utilities|Casting|CastToAI_Blood (UserInterface|GetUserWidgetObject (Variables|Default|Gethealthy))))
  (bind _output_get (Variables|Default|SetAs%20AI%20Blood _asai_blood))
  (Variables|/Game/Other/Cyborg_soldier_V1_ShaoZhiGao/Enemy_AI/AI/AI_Blood.AI_Blood_C|Sethealthy _output_get 5e+01)
  (bind _output_get_2 (Variables|Default|Set存活 true))
  (AI|Components|Blackboard|SetValueasBool (AI|GetBlackboard 0) (Utilities|Name|MakeLiteralName "活着？") _output_get_2))

(event EventGetHit
  ;[1 1 1] 受到伤害的相关判断
  (CallFunction|Hurt))

(event Custom|StopSwordTrace
  (Utilities|Time|ClearandInvalidateTimerbyHandle (Variables|Default|GetSwordTrace)))

(event Custom|StartSwordTrace
  (params (HitFeedback :type Feedback%20Structure))
  (bind _returnvalue (Utilities|Time|SetTimerbyEvent (delegate Custom|SwordTraceLoop) 0.001 true))
  (Variables|Default|SetSwordTrace _returnvalue))

(event Custom|SwordTraceLoop
  (bind (_outhit _returnvalue) (Collision|SphereTraceByChannel (Transformation|GetWorldLocation (Variables|Default|GetTopPoint)) (Transformation|GetWorldLocation (Variables|Default|GetBottomPoint)) 15.0 "TraceTypeQuery4" false 0 "ForDuration" true "(R=1.000000,G=0.000000,B=0.000000,A=1.000000)" "(R=0.000000,G=1.000000,B=0.000000,A=1.000000)" 1.0))
  (if _returnvalue
    (Utilities|FlowControl|DoOnce false :!label _label
      (:Completed
        (bind _asbp_top_down_character (Utilities|Casting|CastToBP_TopDownCharacter (.HitActor (Collision|BreakHitResult _outhit))))
        (Development|PrintString (Utilities|GetDisplayName (.HitActor (Collision|BreakHitResult _outhit))))
        (Default|ChangeHealth (Variables|/Game/Combat_XYH_WeiFu/Blueprints/BP_TopDownCharacter.BP_TopDownCharacter_C|GetBPC_PlayerStats _asbp_top_down_character) (Variables|/Game/3_Blueprint/MonsterStats/BPC_MonsterStats.BPC_MonsterStats_C|GetcurrentDamage (Variables|Default|GetBPC_MonsterStats)) "NewEnumerator1")
        (Default|OnHit (Variables|/Game/Combat_XYH_WeiFu/Blueprints/BP_TopDownCharacter.BP_TopDownCharacter_C|GetBPC_AttackSystem _asbp_top_down_character))
        (Utilities|FlowControl|Delay 0.2)
        (goto _label Reset)))))

(fn ConstructionScript)

(fn ReturnDMGCalculation
  (return (Variables|Default|GetBPC_DamageCalculation)))

(fn GetDamageCalcuationBPC
  (return (Variables|Default|GetBPC_DamageCalculation)))

(fn GetHUD
  (return (Variables|Default|Gethealthy)))

(fn GetIdealRange
  (return 0.0 0.0))

(fn GetMonsterKey
  (return (Variables|Default|GetMonsterKey)))

(fn GetMonsterStats
  (return (Variables|Default|GetBPC_MonsterStats)))

(fn GetPatrolRoutes
  (return 0))

(fn SetMovementSpeed
  (params (movementSpeed :type E_MovementSpeed%20Enum :default "NewEnumerator0"))
  (return 0.0))