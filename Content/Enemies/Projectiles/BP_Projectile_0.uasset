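; Enemy projectile that damages the top-down player character when its box collision hits it.
; Every hit broadcasts ProjectileImpact with the other actor and hit result, then casts that actor to BP_TopDownCharacter.
; Only on a successful cast does it destroy itself, apply Damage through the player stats component's ChangeHealth and call OnHit on the attack system component.
; Other hits leave the projectile undestroyed by this graph.
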(event OnComponentHit(BoxCollision)
  (params (HitComponent :type Primitive%20Component%20Object%20Reference) (OtherActor :type Actor%20Object%20Reference) (OtherComp :type Primitive%20Component%20Object%20Reference) (NormalImpulse :type Vector :default "0, 0, 0") (Hit :type Hit%20Result%20Structure%20%28by%20ref%29))
  ;[1 1 1] Hit
  (Default|CallProjectileImpact OtherActor Hit)
  (bind _asbp_top_down_character (Utilities|Casting|CastToBP_TopDownCharacter OtherActor))
  (Utilities|FlowControl|Sequence
    (:then_0
      (Actor|DestroyActor))
    (:then_1
      (Default|ChangeHealth (Variables|/Game/Combat_XYH_WeiFu/Blueprints/BP_TopDownCharacter.BP_TopDownCharacter_C|GetBPC_PlayerStats _asbp_top_down_character) (Variables|Default|Getdamage) "NewEnumerator1"))
    (:then_2
      (Default|OnHit (Variables|/Game/Combat_XYH_WeiFu/Blueprints/BP_TopDownCharacter.BP_TopDownCharacter_C|GetBPC_AttackSystem _asbp_top_down_character)))))

(event EventBeginPlay
  (|CallParentFunction) ; This node is disabled and will not be called.\nDrag off pins to build functionality.
)

(event EventTick
  (params (DeltaSeconds :type Float%20%28single-precision%29))
  (|CallParentFunction DeltaSeconds) ; This node is disabled and will not be called.\nDrag off pins to build functionality.
)

(fn ConstructionScript
  (|CallParentFunction))