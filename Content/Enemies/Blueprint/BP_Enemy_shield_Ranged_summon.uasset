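; Ranged enemy character that starts with an attached shield actor, fires projectile volleys and summons exploding melee minions.
; The shield absorbs damage until broken, then hits reduce the stats component's health and trigger hit-state reactions; knockback and overlay flash occur either way.
; Attack fires repeated three-arrow volleys after its montage, spawning a nearby minion set to attack the player only when the montage completes uninterrupted.
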(event Custom|ShieldBroken
  (Variables|Default|SetdamageDedection 1.0)
  (Variables|Default|SethasShield false))

(event EventBeginPlay
  (bind _mesh (Variables|Character|GetMesh))
  (bind _returnvalue (Transformation|GetWorldTransform _mesh))
  ;[1 1 1] Init Sheild
  (|CallParentFunction)
  (bind _returnvalue_2 (Game|SpawnActorfromClass "/Game/Enemies/Shield_FX_Functional/Shield_Scifi_01/BluePrint/BP_Master_Shield_01.BP_Master_Shield_01_C" (Math|Transform|MakeTransform (Math|Vector|MakeVector (.x (.location _returnvalue)) (.y (.location _returnvalue)) (+ (.z (.location _returnvalue)) 1e+02)) (.rotation _returnvalue) (.scale _returnvalue)) "Undefined" "MultiplyWithRoot" self 0))
  (Variables|Default|Setshield _returnvalue_2)
  (Transformation|AttachActorToActor _returnvalue_2 self "None" "KeepWorld" "KeepRelative" "KeepRelative" true)
  (Variables|Default|SethasShield true)
  (Utilities|FlowControl|Delay 0.5)
  (Default|ShowShieldBar (Variables|/Game/3_Blueprint/MonsterStats/BPC_MonsterStats.BPC_MonsterStats_C|GetEnemyHUD (Variables|Default|GetBPC_MonsterStats)))
  (bind _asac_enemy_base (Utilities|Casting|CastToAC_Enemy_base (AI|GetAIController self)))
  (Variables|Default|SetAs%20AC%20Enemy%20Base _asac_enemy_base))

(event Collision|EventActorBeginOverlap
  (params (OtherActor :type Actor%20Object%20Reference))
  (|CallParentFunction OtherActor) ; This node is disabled and will not be called.\nDrag off pins to build functionality.
)

(event EventTick
  (params (DeltaSeconds :type Float%20%28single-precision%29))
  (|CallParentFunction DeltaSeconds) ; This node is disabled and will not be called.\nDrag off pins to build functionality.
)

(event EventDeath
  (|CallParentFunction)
  (bind _shield (Variables|Default|GetShield)
    (:then
      (Actor|DestroyActor _shield))
    (:else)))

(event EventChangeHealth
  (params (Damage :type Float%20%28double-precision%29) (IncreaseType :type IncreaseEnum%20Enum :default "NewEnumerator0"))
  (bind _bpc_monsterstats (Variables|Default|GetBPC_MonsterStats))
  ;[1 1 1] ShieldHealthwith Actual HEalth
  (if (Variables|Default|GethasShield)
    (Default|DecreaseHealth (Variables|Default|Getshield) Damage)
    (else
      (Default|ChangeHealth _bpc_monsterstats Damage IncreaseType)
      (if (<= (Variables|/Game/3_Blueprint/MonsterStats/BPC_MonsterStats.BPC_MonsterStats_C|GetCurrentHealth _bpc_monsterstats) 0.0)
        (CallFunction|Death)))))

(event EventGetHit
  (bind _mesh (Variables|Character|GetMesh))
  ;[1 1 1] Gethit
  (Utilities|FlowControl|Sequence
    (:then_1
      (if (> (Variables|/Game/3_Blueprint/MonsterStats/BPC_MonsterStats.BPC_MonsterStats_C|GetCurrentHealth (Variables|Default|GetBPC_MonsterStats)) 0.0)
        (Utilities|FlowControl|DoOnce false :!label _label
          (:Completed
            (Components|Movement|StopMovementImmediately (Variables|Character|GetCharacterMovement))
            (if (Variables|Default|GethasShield)
              _
              (else
                (Default|SetStateasHitState (Variables|Default|GetAs%20AC%20Enemy%20Base))
                (Animation|Montage|PlayMontage (Variables|Character|GetMesh) "/Game/1_Animations/Character/Hit_React/HitReactMonster_UE_Montage.HitReactMonster_UE_Montage" 0.5
                  (:OnCompleted
                    _))))
            (bind _asbp_top_down_character (Utilities|Casting|CastToBP_TopDownCharacter (Game|GetPlayerCharacter 0)))
            (Transformation|SetActorRotation (Math|Rotator|FindLookatRotation (Math|Vector|GetForwardVector (Transformation|GetActorRotation _asbp_top_down_character)) (Transformation|GetActorForwardVector self)))
            (Character|LaunchCharacter (* (Math|Vector|GetForwardVector (Transformation|GetActorRotation _asbp_top_down_character)) 5e+01) false false)
            (goto _label Reset)))
        (else
          (CallFunction|Death))))
    (:then_2
      ;;[1 1 1] vfx
      (Rendering|Material|SetOverlayMaterial _mesh (Variables|Default|GetNew%20Overlay%20Material) :!class /Script/Engine.MeshComponent)
      (Timeline|Timeline_1 PlayFromStart
        (:Finished
          (Timeline|Timeline_2 PlayFromStart
            (:Update
              (Utilities|FlowControl|Delay 0.4)
              (Rendering|Material|SetOverlayMaterial _mesh 0 :!class /Script/Engine.MeshComponent))))))))

(event EventAttack
  ;[1 1 1] Comment
  (Animation|Montage|PlayMontage (Variables|Character|GetMesh) "/Game/Enemies/BasicAnimations/Rifle/Montage_Rifle_Fire.Montage_Rifle_Fire"
    (:OnCompleted
      (Utilities|FlowControl|Sequence
        (:then_0
          (Default|CallAttackFinish :!label _label)
          (for _index (range 0 2)
            (Utilities|FlowControl|Delay 0.1)
            (CallFunction|SpawnBullet (Variables|Default|GetArrow1) 1.8e+03)
            (CallFunction|SpawnBullet (Variables|Default|GetArrow4) 1.8e+03)
            (CallFunction|SpawnBullet (Variables|Default|GetArrow3) 1.8e+03)))
        (:then_1
          (bind _returnvalue (Game|SpawnActorfromClass "/Game/Enemies/Blueprint/BP_Enemy_Melee_Explode.BP_Enemy_Melee_Explode_C" (Math|Conversions|ToTransform(Vector) (.RandomLocation (AI|Navigation|GetRandomReachablePointinRadius (Transformation|GetActorLocation self) 2e+02 0 0))) "Undefined" "MultiplyWithRoot" 0 0))
          (Utilities|IsValid _returnvalue
            (:Is%20Valid
              (Pawn|SpawnDefaultController _returnvalue)
              (bind _asac_enemy_base (Utilities|Casting|CastToAC_Enemy_base (AI|GetAIController _returnvalue)))
              (bind _asbp_top_down_character (Utilities|Casting|CastToBP_TopDownCharacter (Game|GetPlayerCharacter 0)))
              (Default|SetStatesasAttacking _asac_enemy_base _asbp_top_down_character))))))
    (:OnInterrupted
      (goto _label))))

(fn ConstructionScript
  (|CallParentFunction))

(fn ReportDamageEvent
  (bind _asac_enemy_base (Utilities|Casting|CastToAC_Enemy_base (AI|GetAIController self))
    (:then
      (Default|HandleSensedDamage _asac_enemy_base (Game|GetPlayerCharacter 0)))
    (:CastFailed
      (Development|PrintString "Hello"))))

(fn GetMonsterStats
  (return (Variables|Default|GetBPC_MonsterStats)))

(fn GetHUD
  (return (Variables|Default|GetWidget)))

(fn GetIdealRange
  (return 7e+02 7e+02))

(fn SpawnBullet
  (params (Target :type Scene%20Component%20Object%20Reference) (Speed :type Float%20%28double-precision%29))
  (Game|SpawnActorfromClass "/Game/Enemies/Projectiles/BP_Projectile_0.BP_Projectile_0_C" (Math|Transform|MakeTransform (Transformation|GetWorldLocation Target) (Transformation|GetWorldRotation Target) "1.000000,1.000000,1.000000") "Undefined" "OverrideRootScale" self (Variables|/Game/3_Blueprint/MonsterStats/BPC_MonsterStats.BPC_MonsterStats_C|GetcurrentDamage (Variables|Default|GetBPC_MonsterStats)) Speed 0.0 0))

(fn SetMovementSpeed
  (params (movementSpeed :type E_MovementSpeed%20Enum :default "NewEnumerator0"))
  (bind _output_get (Variables|/Script/Engine.CharacterMovementComponent|SetMaxWalkSpeed (Variables|Character|GetCharacterMovement) (Utilities|Select :Index (Utilities|Enum|ByteToEnumE_MovementSpeed movementSpeed) :NewEnumerator0 0.0 :NewEnumerator1 2e+02 :NewEnumerator2 3e+02 :NewEnumerator3 4e+02)))
  (return _output_get))