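; Base melee enemy character with a health widget, AI-facing getters, movement speed presets and a montage attack.
; A timer-driven sphere trace between two sword arrows damages the top-down player.
; GetHit switches the AI controller to hit state, then back to attacking with knockback, or calls Death for montage, delayed destroy and ragdoll attempt.
; Hit shake pairs a bone impulse with timeline-driven physics-blend weight, applied only by a one-shot BeginPlay timer.
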(event Custom|Rogdoll
  ;[1 1 1] Death ragdol
  (Utilities|FlowControl|Delay 2.5)
  (Physics|SetSimulatePhysics (Variables|Character|GetMesh) true))

(event Custom|Death
  ;[1 1 1] Death
  (Utilities|FlowControl|Sequence
    (:then_0
      (Utilities|FlowControl|DoOnce false
        (:Completed
          (Pawn|Components|CharacterMovement|DisableMovement (Variables|Character|GetCharacterMovement))
          (Collision|SetCollisionEnabled (Variables|Character|GetMesh) "NoCollision")
          (Animation|Montage|PlayMontage (Variables|Character|GetMesh) "/Game/Cyborg_soldier_V1_ShaoZhiGao/Enemy_Animation/melee_montage/Frank_RPG_Assassin_Hit_Knockdown_IP_Montage.Frank_RPG_Assassin_Hit_Knockdown_IP_Montage"
            (:then
              (Class|Pawn|DetachfromControllerPendingDestroy)
              (Rendering|SetVisibility (Variables|Default|GetWidget) false false)
              (Utilities|FlowControl|Delay 1.0)
              (Actor|DestroyActor))))))
    (:then_1
      (CallFunction|Rogdoll))))

(event Custom|自定义事件
  (bind _hit_bone_name (Variables|Default|GetHit%20Bone%20Name))
  ;[1 1 1] 骨骼抖动
  (if (> (Variables|Default|GetBlenderWeight) 0.0)
    (Class|SkeletalMeshComponent|SetAllBodiesBelowSimulatePhysics (Variables|Character|GetMesh) _hit_bone_name true true)
    (Class|SkeletalMeshComponent|SetAllBodiesBelowPhysicsBlendWeight (Variables|Character|GetMesh) _hit_bone_name (Variables|Default|GetBlenderWeight) false true)))

(event Custom|SetEnemyBodyShake
  (params (hitBoneName :type Name) (hitDirection :type Vector))
  (bind _mesh (Variables|Character|GetMesh))
  ;[1 1 1] 骨骼抖动
  (if (and (!= hitBoneName "") (!= hitBoneName "pelvis"))
    (Variables|Default|SetHit%20Bone%20Name hitBoneName)
    (else
      (Variables|Default|SetHit%20Bone%20Name "spine_02")))
  (Utilities|FlowControl|Sequence
    (:then_0
      (bind _新建轨道_0 (Timeline|时间轴 PlayFromStart)
        (:Update
          (Variables|Default|SetBlenderWeight _新建轨道_0))
        (:Finished
          (Class|SkeletalMeshComponent|SetAllBodiesPhysicsBlendWeight _mesh 0.0 false)
          (Class|SkeletalMeshComponent|SetAllBodiesSimulatePhysics _mesh false))))
    (:then_1
      (Utilities|FlowControl|Delay 0.06)
      (if (> (Variables|Default|GetBlenderWeight) 0.0)
        (Physics|AddImpulse (Variables|Character|GetMesh) (* hitDirection "10000.000000,10000.000000,10000.000000") (Variables|Default|GetHit%20Bone%20Name) true)))))

(event EventGetHit
  ;[1 1 1] Get hit
  (Utilities|FlowControl|Sequence
    (:then_0
      (bind _asac_enemy_melee_base (Utilities|Casting|CastToAC_Enemy_Melee_base (AI|GetAIController self))))
    (:then_1
      (if (> (Variables|/Game/3_Blueprint/MonsterStats/BPC_MonsterStats.BPC_MonsterStats_C|GetCurrentHealth (Variables|Default|GetBPC_MonsterStats)) 0.0)
        (Utilities|FlowControl|DoOnce false :!label _label
          (:Completed
            (Components|Movement|StopMovementImmediately (Variables|Character|GetCharacterMovement))
            (Default|SetStateasHitState _asac_enemy_melee_base)
            (Animation|Montage|PlayMontage (Variables|Character|GetMesh) "/Game/Cyborg_soldier_V1_ShaoZhiGao/Enemy_Animation/melee_montage/Frank_RPG_Assassin_Hit02_Montage.Frank_RPG_Assassin_Hit02_Montage" 0.5
              (:OnCompleted
                (Default|SetStatesasAttacking _asac_enemy_melee_base (Game|GetPlayerCharacter 0))
                (bind _asbp_top_down_character (Utilities|Casting|CastToBP_TopDownCharacter (Game|GetPlayerCharacter 0)))
                (Transformation|SetActorRotation (Math|Rotator|FindLookatRotation (Math|Vector|GetForwardVector (Transformation|GetActorRotation _asbp_top_down_character)) (Transformation|GetActorForwardVector self)))
                (Character|LaunchCharacter (* (Math|Vector|GetForwardVector (Transformation|GetActorRotation _asbp_top_down_character)) 5e+01) false false)
                (goto _label Reset)))))
        (else
          (CallFunction|Death))))
    (:then_2
      (Development|PrintString (Utilities|String|ToString(Float) (Variables|/Game/3_Blueprint/MonsterStats/BPC_MonsterStats.BPC_MonsterStats_C|GetCurrentHealth (Variables|Default|GetBPC_MonsterStats)))))))

(event Collision|EventActorBeginOverlap
  (params (OtherActor :type Actor%20Object%20Reference)))

(event EventTick
  (params (DeltaSeconds :type Float%20%28single-precision%29)))

(event EventChangeHealth
  (params (MonsterStats :type BPC%20Monster%20Stats%20Object%20Reference) (Damage :type Float%20%28double-precision%29) (IncreaseType :type IncreaseEnum%20Enum :default "NewEnumerator0"))
  (Default|ChangeHealth MonsterStats Damage IncreaseType))

(event EventBeginPlay
  (bind _bpc_monsterstats (Variables|Default|GetBPC_MonsterStats))
  ;[1 1 1] 骨骼抖动
  (Utilities|FlowControl|Sequence
    (:then_0
      (bind _asenemy_hp (Utilities|Casting|CastToEnemy_Hp (UserInterface|GetWidget (Variables|Default|GetWidget))))
      (Progress|SetPercent (Variables|/Game/Enemies/UI/Enemy_Hp.Enemy_Hp_C|GetHP_bar _asenemy_hp) (/ (Variables|/Game/3_Blueprint/MonsterStats/BPC_MonsterStats.BPC_MonsterStats_C|GetCurrentHealth _bpc_monsterstats) (Variables|/Game/3_Blueprint/MonsterStats/BPC_MonsterStats.BPC_MonsterStats_C|GetMaxHealth _bpc_monsterstats))))
    (:then_1
      (Utilities|Time|SetTimerbyEvent (delegate Custom|自定义事件) 0.016667))))

(event Custom|Attack
  (Animation|Montage|PlayMontage (Variables|Character|GetMesh) "/Game/Cyborg_soldier_V1_ShaoZhiGao/Enemy_Animation/melee_montage/Frank_RPG_Assassin_Combo01_2_IP_Montage.Frank_RPG_Assassin_Combo01_2_IP_Montage"
    (:OnCompleted
      _)
    (:OnInterrupted
      _))
  (Default|CallAttackFinish))

(event Custom|StopSwordTrace
  (Utilities|Time|ClearandInvalidateTimerbyHandle (Variables|Default|GetSword%20Trace)))

(event Custom|StartSwordTrace
  (params (HitFeedback :type Feedback%20Structure))
  (bind _returnvalue (Utilities|Time|SetTimerbyEvent (delegate Custom|SwordTraceLoop) 0.0001 true))
  (Variables|Default|SetSword%20Trace _returnvalue))

(event Custom|SwordTraceLoop
  (bind (_outhit _returnvalue) (Collision|SphereTraceByChannel (Transformation|GetWorldLocation (Variables|Default|GetArrow1)) (Transformation|GetWorldLocation (Variables|Default|GetArrow2)) 15.0 "TraceTypeQuery4" false 0 "ForDuration" true "(R=1.000000,G=0.000000,B=0.000000,A=1.000000)" "(R=0.000000,G=1.000000,B=0.000000,A=1.000000)" 1.0))
  (if _returnvalue
    (Utilities|FlowControl|DoOnce false :!label _label
      (:Completed
        (bind _asbp_top_down_character (Utilities|Casting|CastToBP_TopDownCharacter (.HitActor (Collision|BreakHitResult _outhit))))
        (Development|PrintString (Utilities|GetDisplayName (.HitActor (Collision|BreakHitResult _outhit))))
        (Default|ChangeHealth (Variables|/Game/Combat_XYH_WeiFu/Blueprints/BP_TopDownCharacter.BP_TopDownCharacter_C|GetBPC_PlayerStats _asbp_top_down_character) (Variables|/Game/3_Blueprint/MonsterStats/BPC_MonsterStats.BPC_MonsterStats_C|GetcurrentDamage (Variables|Default|GetBPC_MonsterStats)) "NewEnumerator1")
        (Default|OnHit (Variables|/Game/Combat_XYH_WeiFu/Blueprints/BP_TopDownCharacter.BP_TopDownCharacter_C|GetBPC_AttackSystem _asbp_top_down_character))
        (Utilities|FlowControl|Delay 0.2)
        (goto _label Reset)))))

(fn ConstructionScript)

(fn GetDamageCalcuationBPC
  (return (Variables|Default|GetBPC_DamageCalculation)))

(fn GetHUD
  (return (Variables|Default|GetWidget)))

(fn GetIdealRange
  (return 1.5e+02 4e+02))

(fn GetMonsterKey
  (return (Variables|Default|GetMonsterKey)))

(fn GetMonsterStats
  (return (Variables|Default|GetBPC_MonsterStats)))

(fn GetPatrolRoutes
  (return (Variables|ai|GetpatrolRoutes)))

(fn SetMovementSpeed
  (params (movementSpeed :type E_MovementSpeed%20Enum :default "NewEnumerator0"))
  (bind _output_get (Variables|/Script/Engine.CharacterMovementComponent|SetMaxWalkSpeed (Variables|Character|GetCharacterMovement) (Utilities|Select :Index movementSpeed :NewEnumerator0 0.0 :NewEnumerator1 3e+02 :NewEnumerator2 4e+02 :NewEnumerator3 5e+02)))
  (return _output_get))