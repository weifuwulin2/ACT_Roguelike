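; Boss enemy Blueprint for a top-down game, driven by AC_Enemy_boss1, with sword, dash, combo and bullet-hell attacks.
; Attack events chain montages with player re-focusing and report completion through dispatchers, while ranged events fire timed projectile volleys from arrow components.
; Hits flash an overlay material, reveal the boss HP bar and shift the AI to second and final states at health thresholds.
; A looping-timer sphere trace applies sword damage once per swing.
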(event Custom|ComboAttack
  (bind _duration (Variables|Default|GetDuration))
  ;[1 1 1] ComboAttack
  (CallFunction|SetFocus)
  (Animation|Montage|PlayMontage (Variables|Character|GetMesh) "/Game/1_Animations/Enemies/ShieldEnemy/Shield_Attack_Anim.Shield_Attack_Anim"
    (:OnCompleted
      (Utilities|FlowControl|Delay _duration)
      (CallFunction|SetFocus)
      (Animation|Montage|PlayMontage (Variables|Character|GetMesh) "/Game/1_Animations/Enemies/ShieldEnemy/Shield_Attack_Anim.Shield_Attack_Anim"
        (:OnCompleted
          (Utilities|FlowControl|Delay _duration)
          (CallFunction|SetFocus)
          (Animation|Montage|PlayMontage (Variables|Character|GetMesh) "/Game/1_Animations/Enemies/ShieldEnemy/Shield_Attack_Anim.Shield_Attack_Anim"
            (:OnCompleted
              (Utilities|FlowControl|Delay 0.5)
              (CallFunction|SetFocus)
              (Animation|Montage|PlayMontage (Variables|Character|GetMesh) "/Game/1_Animations/Enemies/Boss/Boss_Ranged_Anim_Montage.Boss_Ranged_Anim_Montage"
                (:OnCompleted
                  _)
                (:OnInterrupted
                  _))
              (Default|CallAttackFinish))))))))

(event Custom|PlayEncounterAnimation
  ;[1 1 1] EncounterAnimation
  (Animation|Montage|PlayMontage (Variables|Character|GetMesh) "/Game/1_Animations/Enemies/Boss/Montage_Unsheath_Sword.Montage_Unsheath_Sword"
    (:OnCompleted
      (Rendering|SetVisibility (Variables|Default|GetSK_Katana_01_A) true false))
    (:OnInterrupted
      _))
  (Default|CallEncounterAnimationFinished))

(event Custom|RangedAttack_Final
  ;[1 1 1] BulletHell
  (CallFunction|SpawnBullet 1.8e+03 (Variables|Default|GetArrow5))
  (CallFunction|SpawnBullet 1.8e+03 (Variables|Default|GetArrow6))
  (CallFunction|SpawnBullet 1.8e+03 (Variables|Default|GetArrow7))
  (CallFunction|SpawnBullet 1.8e+03 (Variables|Default|GetArrow8))
  (CallFunction|SpawnBullet 1.8e+03 (Variables|Default|GetArrow9))
  (Utilities|FlowControl|Delay 0.3)
  (CallFunction|SpawnBullet 1.8e+03 (Variables|Default|GetArrow5))
  (CallFunction|SpawnBullet 1.8e+03 (Variables|Default|GetArrow6))
  (CallFunction|SpawnBullet 1.8e+03 (Variables|Default|GetArrow7))
  (CallFunction|SpawnBullet 1.8e+03 (Variables|Default|GetArrow8))
  (CallFunction|SpawnBullet 1.8e+03 (Variables|Default|GetArrow9))
  (Utilities|FlowControl|Delay 0.3)
  (CallFunction|SpawnBullet 1.8e+03 (Variables|Default|GetArrow5))
  (CallFunction|SpawnBullet 1.8e+03 (Variables|Default|GetArrow6))
  (CallFunction|SpawnBullet 1.8e+03 (Variables|Default|GetArrow7))
  (CallFunction|SpawnBullet 1.8e+03 (Variables|Default|GetArrow8))
  (CallFunction|SpawnBullet 1.8e+03 (Variables|Default|GetArrow9)))

(event Custom|ComboAttack_Final
  ;[1 1 1] FinalState
  (Animation|Montage|PlayMontage (Variables|Character|GetMesh) "/Game/1_Animations/Enemies/Boss/Boss_Combo2.Boss_Combo2" 0.7
    (:OnCompleted
      _)
    (:OnInterrupted
      _))
  (CallFunction|SetFocus)
  (Utilities|FlowControl|Delay (Variables|Default|GetDuration))
  (Animation|Montage|PlayMontage (Variables|Character|GetMesh) "/Game/1_Animations/Enemies/ShieldEnemy/Shield_Attack_Anim.Shield_Attack_Anim"
    (:OnCompleted
      (Utilities|FlowControl|Delay (Variables|Default|GetDuration))
      (CallFunction|SetFocus)
      (Animation|Montage|PlayMontage (Variables|Character|GetMesh) "/Game/1_Animations/Enemies/ShieldEnemy/Shield_Attack_Anim.Shield_Attack_Anim"
        (:OnCompleted
          (Utilities|FlowControl|Delay 0.5))
        (:OnInterrupted
          _))
      (Animation|Montage|PlayMontage (Variables|Character|GetMesh) "/Game/1_Animations/Enemies/Boss/Boss_Combo2.Boss_Combo2" 0.7
        (:OnCompleted
          (Utilities|FlowControl|Delay 0.5)
          (CallFunction|SetFocus)
          (Animation|Montage|PlayMontage (Variables|Character|GetMesh) "/Game/1_Animations/Enemies/Boss/Boss_Ranged_Anim_Montage_1.Boss_Ranged_Anim_Montage_1"
            (:OnCompleted
              _)
            (:OnInterrupted
              _))
          (Default|CallAttackFinish))))))

(event Custom|RangedAttack
  ;[1 1 1] BulletHell
  (CallFunction|SpawnBullet 1.8e+03 (Variables|Default|GetArrow5))
  (CallFunction|SpawnBullet 1.8e+03 (Variables|Default|GetArrow6))
  (CallFunction|SpawnBullet 1.8e+03 (Variables|Default|GetArrow7))
  (CallFunction|SpawnBullet 1.8e+03 (Variables|Default|GetArrow8))
  (CallFunction|SpawnBullet 1.8e+03 (Variables|Default|GetArrow9))
  (Utilities|FlowControl|Delay 0.3)
  (CallFunction|SpawnBullet 1.8e+03 (Variables|Default|GetArrow5))
  (CallFunction|SpawnBullet 1.8e+03 (Variables|Default|GetArrow6))
  (CallFunction|SpawnBullet 1.8e+03 (Variables|Default|GetArrow7))
  (CallFunction|SpawnBullet 1.8e+03 (Variables|Default|GetArrow8))
  (CallFunction|SpawnBullet 1.8e+03 (Variables|Default|GetArrow9)))

(event Custom|Attack_Dash
  ;[1 1 1] BossAttack
  (Animation|Montage|PlayMontage (Variables|Character|GetMesh) "/Game/1_Animations/Enemies/ShieldEnemy/Shield_Attack_Anim.Shield_Attack_Anim"
    (:OnCompleted
      _)
    (:OnInterrupted
      _))
  (Default|CallAttackFinish))

(event EventBeginPlay
  (bind _enemy_weapon (Variables|Default|GetEnemy_Weapon))
  ;[1 1 1] Init
  (|CallParentFunction)
  (Rendering|SetVisibility (Variables|Default|GetSK_Katana_01_A) false false)
  (Rendering|SetVisibility _enemy_weapon false false)
  (Collision|SetCollisionEnabled _enemy_weapon "NoCollision")
  (bind _asbp_top_down_character (Utilities|Casting|CastToBP_TopDownCharacter (Game|GetPlayerCharacter 0)))
  (Variables|Default|SetAs%20BP%20Top%20Down%20Character _asbp_top_down_character)
  (bind _asac_enemy_boss_1 (Utilities|Casting|CastToAC_Enemy_boss1 (AI|GetAIController self)))
  (Variables|Default|SetAs%20AC%20Enemy%20Boss%201 _asac_enemy_boss_1)
  (Rendering|SetVisibility (Variables|Default|GetWidget) false false))

(event EventGetHit
  (bind _bpc_monsterstats (Variables|Default|GetBPC_MonsterStats))
  (bind _mesh (Variables|Character|GetMesh))
  (bind _bpc_monsterstats_2 (Variables|Default|GetBPC_MonsterStats))
  ;[1 1 1] BossHit
  (Utilities|FlowControl|Sequence
    (:then_0
      (if (> (Variables|/Game/3_Blueprint/MonsterStats/BPC_MonsterStats.BPC_MonsterStats_C|GetCurrentHealth (Variables|Default|GetBPC_MonsterStats)) 0.0)
        (Utilities|FlowControl|DoOnce false :!label _label
          (:Completed
            (Components|Movement|StopMovementImmediately (Variables|Character|GetCharacterMovement))
            (bind _asbp_top_down_character (Utilities|Casting|CastToBP_TopDownCharacter (Game|GetPlayerCharacter 0)))
            (Transformation|SetActorRotation (Math|Rotator|FindLookatRotation (Math|Vector|GetForwardVector (Transformation|GetActorRotation _asbp_top_down_character)) (Transformation|GetActorForwardVector self)))
            (goto _label Reset)))
        (else
          (CallFunction|Death))))
    (:then_1
      ;;[1 1 1] vfx
      (Rendering|Material|SetOverlayMaterial _mesh (Variables|Default|GetNew%20Overlay%20Material) :!class /Script/Engine.MeshComponent)
      (Timeline|Timeline_1 PlayFromStart
        (:Finished
          (Timeline|Timeline_2 PlayFromStart
            (:Finished
              (Utilities|FlowControl|Delay 0.2)
              (Rendering|Material|SetOverlayMaterial _mesh 0 :!class /Script/Engine.MeshComponent))))))
    (:then_2
      ;;[1 1 1] BossStateChangeBasedOnHP
      (if (<= (/ (Variables|/Game/3_Blueprint/MonsterStats/BPC_MonsterStats.BPC_MonsterStats_C|GetCurrentHealth _bpc_monsterstats) (Variables|/Game/3_Blueprint/MonsterStats/BPC_MonsterStats.BPC_MonsterStats_C|GetMaxHealth _bpc_monsterstats)) 0.66)
        (Default|SetStateasSecondState (Variables|Default|GetAs%20AC%20Enemy%20Boss%201) (Variables|Default|GetAs%20BP%20Top%20Down%20Character))
        (if (<= (/ (Variables|/Game/3_Blueprint/MonsterStats/BPC_MonsterStats.BPC_MonsterStats_C|GetCurrentHealth _bpc_monsterstats_2) (Variables|/Game/3_Blueprint/MonsterStats/BPC_MonsterStats.BPC_MonsterStats_C|GetMaxHealth _bpc_monsterstats_2)) 0.3)
          (Default|SetStateasFinalState (Variables|Default|GetAs%20AC%20Enemy%20Boss%201) (Variables|Default|GetAs%20BP%20Top%20Down%20Character)))))
    (:then_3
      (Widget|SetVisibility (Variables|/Game/3_Blueprint/UI/WB_HUD.WB_HUD_C|GetBoss_HP (Variables|/Game/3_Blueprint/PlayerStats/BPC_PlayerStats.BPC_PlayerStats_C|GetplayerHUD (Variables|/Game/Combat_XYH_WeiFu/Blueprints/BP_TopDownCharacter.BP_TopDownCharacter_C|GetBPC_PlayerStats (Variables|Default|GetAs%20BP%20Top%20Down%20Character)))) "Visible"))))

(event EventStartSwordTrace
  (params (HitFeedback :type Feedback%20Structure))
  ;[1 1 1] BOSS: ATTACK DETECTION
  (bind _returnvalue (Utilities|Time|SetTimerbyEvent (delegate EventSwordTraceLoop) 0.001 true))
  (Variables|Default|SetSword%20Trace _returnvalue))

(event EventSwordTraceLoop
  (bind _bpc_monsterstats (Variables|Default|GetBPC_MonsterStats))
  ;[1 1 1] BOSS: ATTACK DETECTION
  (bind (_outhit _returnvalue) (Collision|SphereTraceByChannel (Transformation|GetWorldLocation (Variables|Default|GetArrow3)) (Transformation|GetWorldLocation (Variables|Default|GetArrow4)) 1e+02 "TraceTypeQuery4" false 0 "ForDuration" true "(R=1.000000,G=0.000000,B=0.000000,A=1.000000)" "(R=0.000000,G=1.000000,B=0.000000,A=1.000000)" 1.0))
  (if _returnvalue
    (Utilities|FlowControl|DoOnce false
      (:Completed
        (bind _asbp_top_down_character (Utilities|Casting|CastToBP_TopDownCharacter (.HitActor (Collision|BreakHitResult _outhit))))
        (Default|OnHit _asbp_top_down_character (Variables|/Game/3_Blueprint/MonsterStats/BPC_MonsterStats.BPC_MonsterStats_C|GetAttackStraight _bpc_monsterstats))
        (Default|ChangeHealth (Variables|/Game/Combat_XYH_WeiFu/Blueprints/BP_TopDownCharacter.BP_TopDownCharacter_C|GetBPC_PlayerStats _asbp_top_down_character) (Variables|/Game/3_Blueprint/MonsterStats/BPC_MonsterStats.BPC_MonsterStats_C|GetcurrentDamage _bpc_monsterstats) "NewEnumerator1")))))

(event EventStopSwordTrace
  (bind _bpc_monsterstats (Variables|Default|GetBPC_MonsterStats))
  ;[1 1 1] BOSS: ATTACK DETECTION
  (Utilities|Time|ClearandInvalidateTimerbyHandle (Variables|Default|GetSword%20Trace))
  (Utilities|FlowControl|DoOnce false) ; enters at Reset
)

(event EventAttack
  ;[1 1 1] BossAttack
  (Animation|Montage|PlayMontage (Variables|Character|GetMesh) "/Game/1_Animations/Enemies/Boss/BossAttack_01.BossAttack_01"
    (:OnCompleted
      _)
    (:OnInterrupted
      _))
  (Default|CallAttackFinish))

(event EventDeath
  (|CallParentFunction))

(fn ConstructionScript
  (Components|SkinnedMesh|SetLeaderPoseComponent (Variables|Default|GetSK_BELT_SHEAT_LOD0) (Variables|Character|GetMesh) false false))

(fn GetIdealRange
  (return 5e+02 5e+02))

(fn SetMovementSpeed
  (params (movementSpeed :type E_MovementSpeed%20Enum :default "NewEnumerator0"))
  (bind _output_get (Variables|/Script/Engine.CharacterMovementComponent|SetMaxWalkSpeed (Variables|Character|GetCharacterMovement) (Utilities|Select :Index (Utilities|Enum|ByteToEnumE_MovementSpeed movementSpeed) :NewEnumerator0 0.0 :NewEnumerator1 4e+02 :NewEnumerator2 5e+02 :NewEnumerator3 6e+02)))
  (return _output_get))

(fn SpawnBullet
  (params (Speed :type Float%20%28double-precision%29) (Target :type Scene%20Component%20Object%20Reference))
  (Game|SpawnActorfromClass "/Game/Enemies/Projectiles/BP_Projectile_0.BP_Projectile_0_C" (Math|Transform|MakeTransform (Transformation|GetWorldLocation Target) (Transformation|GetWorldRotation Target) "1.000000,1.000000,1.000000") "Undefined" "OverrideRootScale" self (Variables|/Game/3_Blueprint/MonsterStats/BPC_MonsterStats.BPC_MonsterStats_C|GetcurrentDamage (Variables|Default|GetBPC_MonsterStats)) Speed 0.0 0))

(fn SetFocus
  (AI|SetFocus (Variables|Default|GetAs%20AC%20Enemy%20Boss%201) (Variables|Default|GetAs%20BP%20Top%20Down%20Character)))

(fn ClearFocus
  (AI|ClearFocus (Variables|Default|GetAs%20AC%20Enemy%20Boss%201)))