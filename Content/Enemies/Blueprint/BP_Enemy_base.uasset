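; Base enemy character that handles health, hit reactions and death, with getters for stats, patrol routes, combat ranges and walk-speed presets.
; GetHit sets the AI controller's hit state, plays a montage, knocks the enemy back and pulses a refraction overlay.
; Zero health triggers ragdoll, hides the HP widget and destroys the actor after a delay.
; Attack is a print stub, and the bone-shake physics blend timer is unwired.
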(event Custom|Rogdoll
  ;[1 1 1] Death ragdol
  (Physics|SetSimulatePhysics (Variables|Character|GetMesh) true))

(event Custom|Death
  ;[1 1 1] Death
  (Utilities|FlowControl|Sequence
    (:then_0
      (Utilities|FlowControl|DoOnce false
        (:Completed
          (CallFunction|Rogdoll)
          (Rendering|SetVisibility (Variables|Default|GetWidget) false false)
          (Utilities|FlowControl|Delay 1.0)
          (Actor|DestroyActor))))
    (:then_1
      (Development|PrintString "die"))))

(event Custom|Attack
  (Development|PrintString "Do attack"))

(event Custom|SetEnemyBodyShake
  (params (hitBoneName :type Name) (hitDirection :type Vector))
  (bind _mesh (Variables|Character|GetMesh))
  ;[1 1 1] 骨骼抖动
  (if (and (!= hitBoneName "") (!= hitBoneName "pelvis"))
    (Variables|Default|SetHit%20Bone%20Name hitBoneName)
    (else
      (Variables|Default|SetHit%20Bone%20Name "spine_02")))
  (Utilities|FlowControl|Sequence
    (:then_0
      (bind _新建轨道_0 (Timeline|时间轴 PlayFromStart)
        (:Update
          (Variables|Default|SetBlenderWeight _新建轨道_0))
        (:Finished
          (Class|SkeletalMeshComponent|SetAllBodiesPhysicsBlendWeight _mesh 0.0 false)
          (Class|SkeletalMeshComponent|SetAllBodiesSimulatePhysics _mesh false))))
    (:then_1
      (Utilities|FlowControl|Delay 0.06)
      (if (> (Variables|Default|GetBlenderWeight) 0.0)
        (Physics|AddImpulse (Variables|Character|GetMesh) (* hitDirection "10000.000000,10000.000000,10000.000000") (Variables|Default|GetHit%20Bone%20Name) true)))))

(event EventGetHit
  (bind _mesh (Variables|Character|GetMesh))
  (bind _mesh_2 (Variables|Character|GetMesh))
  ;[1 1 1] Get hit
  (Utilities|FlowControl|Sequence
    (:then_0
      (bind _asac_enemy_base (Utilities|Casting|CastToAC_Enemy_base (AI|GetAIController self))))
    (:then_1
      (if (> (Variables|/Game/3_Blueprint/MonsterStats/BPC_MonsterStats.BPC_MonsterStats_C|GetCurrentHealth (Variables|Default|GetBPC_MonsterStats)) 0.0)
        (Utilities|FlowControl|DoOnce false :!label _label
          (:Completed
            (Components|Movement|StopMovementImmediately (Variables|Character|GetCharacterMovement))
            (Default|SetStateasHitState _asac_enemy_base)
            (Animation|Montage|PlayMontage (Variables|Character|GetMesh) "/Game/1_Animations/Character/Hit_React/HitReactMonster_UE_Montage.HitReactMonster_UE_Montage" 0.5
              (:then
                (bind _asbp_top_down_character (Utilities|Casting|CastToBP_TopDownCharacter (Game|GetPlayerCharacter 0)))
                (Transformation|SetActorRotation (Math|Rotator|FindLookatRotation (Math|Vector|GetForwardVector (Transformation|GetActorRotation _asbp_top_down_character)) (Transformation|GetActorForwardVector self)))
                (Character|LaunchCharacter (* (Math|Vector|GetForwardVector (Transformation|GetActorRotation _asbp_top_down_character)) 2e+02) false false)
                (goto _label Reset)))))
        (else
          (CallFunction|Death))))
    (:then_2
      ;[1 1 1] vfx
      (Rendering|Material|SetOverlayMaterial _mesh (Variables|Default|GetNew%20Overlay%20Material) :!class /Script/Engine.MeshComponent)
      (bind _strength_refraction (Timeline|Timeline PlayFromStart)
        (:Update
          (Rendering|Material|SetScalarParameterValueonMaterials _mesh_2 "Strength_Refraction" _strength_refraction))
        (:Finished
          (bind _strength_refraction_2 (Timeline|Timeline_0 PlayFromStart)
            (:Update
              (Rendering|Material|SetScalarParameterValueonMaterials _mesh_2 "Strength_Refraction" _strength_refraction_2)
              (Utilities|FlowControl|Delay 0.2)
              (Rendering|Material|SetOverlayMaterial _mesh 0 :!class /Script/Engine.MeshComponent))))))))

(event Collision|EventActorBeginOverlap
  (params (OtherActor :type Actor%20Object%20Reference)))

(event EventTick
  (params (DeltaSeconds :type Float%20%28single-precision%29)))

(event EventChangeHealth
  (params (Damage :type Float%20%28double-precision%29) (IncreaseType :type IncreaseEnum%20Enum :default "NewEnumerator0"))
  (bind _bpc_monsterstats (Variables|Default|GetBPC_MonsterStats))
  (Default|ChangeHealth _bpc_monsterstats Damage IncreaseType)
  (if (<= (Variables|/Game/3_Blueprint/MonsterStats/BPC_MonsterStats.BPC_MonsterStats_C|GetCurrentHealth _bpc_monsterstats) 0.0)
    (CallFunction|Death)))

(event Custom|自定义事件
  (bind _hit_bone_name (Variables|Default|GetHit%20Bone%20Name))
  ;[1 1 1] Initialization
  (if (> (Variables|Default|GetBlenderWeight) 0.0)
    (Class|SkeletalMeshComponent|SetAllBodiesBelowSimulatePhysics (Variables|Character|GetMesh) _hit_bone_name true true)
    (Class|SkeletalMeshComponent|SetAllBodiesBelowPhysicsBlendWeight (Variables|Character|GetMesh) _hit_bone_name (Variables|Default|GetBlenderWeight) false true)))

(event EventBeginPlay
  (bind _bpc_monsterstats (Variables|Default|GetBPC_MonsterStats))
  ;[1 1 1] Initialization
  (Utilities|FlowControl|Sequence
    (:then_0
      (bind _asenemy_hp (Utilities|Casting|CastToEnemy_Hp (UserInterface|GetWidget (Variables|Default|GetWidget))))
      (Progress|SetPercent (Variables|/Game/Enemies/UI/Enemy_Hp.Enemy_Hp_C|GetHP_bar _asenemy_hp) (/ (Variables|/Game/3_Blueprint/MonsterStats/BPC_MonsterStats.BPC_MonsterStats_C|GetCurrentHealth _bpc_monsterstats) (Variables|/Game/3_Blueprint/MonsterStats/BPC_MonsterStats.BPC_MonsterStats_C|GetMaxHealth _bpc_monsterstats))))))

(fn ConstructionScript)

(fn GetDamageCalcuationBPC
  (return (Variables|Default|GetBPC_DamageCalculation)))

(fn GetHUD
  (return (Variables|Default|GetWidget)))

(fn GetIdealRange
  (return 1.5e+02 4e+02))

(fn GetMonsterKey
  (return (Variables|Default|GetMonsterKey)))

(fn GetMonsterStats
  (return (Variables|Default|GetBPC_MonsterStats)))

(fn GetPatrolRoutes
  (return (Variables|ai|GetpatrolRoutes)))

(fn SetMovementSpeed
  (params (movementSpeed :type E_MovementSpeed%20Enum :default "NewEnumerator0"))
  (bind _output_get (Variables|/Script/Engine.CharacterMovementComponent|SetMaxWalkSpeed (Variables|Character|GetCharacterMovement) (Utilities|Select :Index (Utilities|Enum|ByteToEnumE_MovementSpeed movementSpeed) :NewEnumerator0 0.0 :NewEnumerator1 3e+02 :NewEnumerator2 4e+02 :NewEnumerator3 5e+02)))
  (return _output_get))