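; Shielded enemy that spawns and attaches a BP_Master_Shield_01 actor on BeginPlay and destroys it on death.
; Incoming damage is scaled by a multiplier, which ShieldBroken resets to full while clearing the shield flag.
; Hits knock it along the player's forward vector, preceded by a hit state and montage only when unshielded, or trigger Death at zero health.
; ReportDamageEvent passes the player to the AI controller as the sensed damage source.
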(event Custom|ShieldBroken
  (Variables|Default|SetdamageDedection 1.0)
  (Variables|Default|SethasShield false))

(event EventBeginPlay
  (bind _mesh (Variables|Character|GetMesh))
  (bind _returnvalue (Transformation|GetWorldTransform _mesh))
  (|CallParentFunction)
  (bind _returnvalue_2 (Game|SpawnActorfromClass "/Game/Cyborg_soldier_V1_ShaoZhiGao/Shield_FX_Functional/Shield_Scifi_01/BluePrint/BP_Master_Shield_01.BP_Master_Shield_01_C" (Math|Transform|MakeTransform (Math|Vector|MakeVector (.x (.location _returnvalue)) (.y (.location _returnvalue)) (+ (.z (.location _returnvalue)) 1e+02)) (.rotation _returnvalue) (.scale _returnvalue)) "Undefined" "MultiplyWithRoot" self 0))
  (bind _output_get (Variables|Default|Setshield _returnvalue_2))
  (Transformation|AttachActorToActor _output_get self "None" "KeepWorld" "KeepRelative" "KeepRelative" true)
  (Variables|Default|SethasShield true))

(event Collision|EventActorBeginOverlap
  (params (OtherActor :type Actor%20Object%20Reference))
  (|CallParentFunction OtherActor) ; This node is disabled and will not be called.\nDrag off pins to build functionality.
)

(event EventTick
  (params (DeltaSeconds :type Float%20%28single-precision%29))
  (|CallParentFunction DeltaSeconds) ; This node is disabled and will not be called.\nDrag off pins to build functionality.
)

(event EventDeath
  (|CallParentFunction)
  (bind _shield (Variables|Default|GetShield)
    (:then
      (Actor|DestroyActor _shield))
    (:else)))

(event EventChangeHealth
  (params (MonsterStats :type BPC%20Monster%20Stats%20Object%20Reference) (Damage :type Float%20%28double-precision%29) (IncreaseType :type IncreaseEnum%20Enum :default "NewEnumerator0"))
  (Default|ChangeHealth MonsterStats (* Damage (Variables|Default|GetdamageDedection)) IncreaseType)
  (Development|PrintString (Utilities|String|ToString(Float) (Variables|/Game/3_Blueprint/MonsterStats/BPC_MonsterStats.BPC_MonsterStats_C|GetCurrentHealth (Variables|Default|GetBPC_MonsterStats)))))

(event EventGetHit
  (Utilities|FlowControl|Sequence
    (:then_0
      (bind _asac_enemy_base (Utilities|Casting|CastToAC_Enemy_base (AI|GetAIController self))))
    (:then_1
      (if (> (Variables|/Game/3_Blueprint/MonsterStats/BPC_MonsterStats.BPC_MonsterStats_C|GetCurrentHealth (Variables|Default|GetBPC_MonsterStats)) 0.0)
        (Utilities|FlowControl|DoOnce false :!label _label
          (:Completed
            (Components|Movement|StopMovementImmediately (Variables|Character|GetCharacterMovement))
            (if (Variables|Default|GethasShield)
              _
              (else
                (Default|SetStateasHitState _asac_enemy_base)
                (Animation|Montage|PlayMontage (Variables|Character|GetMesh) "/Game/1_Animations/Character/Hit_React/HitReactMonster_UE_Montage.HitReactMonster_UE_Montage" 0.5
                  (:OnCompleted
                    _))))
            (bind _asbp_top_down_character (Utilities|Casting|CastToBP_TopDownCharacter (Game|GetPlayerCharacter 0)))
            (Transformation|SetActorRotation (Math|Rotator|FindLookatRotation (Math|Vector|GetForwardVector (Transformation|GetActorRotation _asbp_top_down_character)) (Transformation|GetActorForwardVector self)))
            (Character|LaunchCharacter (* (Math|Vector|GetForwardVector (Transformation|GetActorRotation _asbp_top_down_character)) 5e+01) false false)
            (goto _label Reset)))
        (else
          (CallFunction|Death))))))

(fn ConstructionScript
  (|CallParentFunction))

(fn ReportDamageEvent
  (bind _asac_enemy_base (Utilities|Casting|CastToAC_Enemy_base (AI|GetAIController self)))
  (Default|HandleSensedDamage _asac_enemy_base (Game|GetPlayerCharacter 0)))