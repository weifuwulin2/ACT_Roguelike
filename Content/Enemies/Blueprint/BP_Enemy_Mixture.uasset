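; Mixture enemy Blueprint that fights with sword or rifle, chosen by its AI controller's blackboard state.
; GetHit switches it to ranged state, mesh and anim class, repeating this at half health or below.
; Hits also trigger death, or a stagger montage with knockback along the player's facing.
; Attack plays the matching montage; rifle fire spawns a player-aimed projectile when the montage completes or is interrupted.
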(event EventBeginPlay
  (|CallParentFunction))

(event EventGetHit
  (bind _bpc_monsterstats (Variables|Default|GetBPC_MonsterStats))
  (Utilities|FlowControl|Sequence
    (:then_0
      (bind _asac_enemy_base (Utilities|Casting|CastToAC_Enemy_base (AI|GetAIController self)))
      (bind _asactor (Utilities|Casting|CastToActor (AI|Components|Blackboard|GetValueasObject (Variables|/Script/AIModule.AIController|GetBlackboard _asac_enemy_base) (Utilities|Name|MakeLiteralName "AttackTarget")) :!label _label))
      (Default|SetStateasSwitchRangedAttack _asac_enemy_base _asactor)
      (Components|SkeletalMesh|SetSkeletalMeshAsset (Variables|Character|GetMesh) (Variables|Default|GetskeletalMesh))
      (Class|SkeletalMeshComponent|SetAnimClass (Variables|Character|GetMesh) (Utilities|GetClass (Variables|Default|GetanimBlueprint_ranged))))
    (:then_1
      (if (> (Variables|/Game/3_Blueprint/MonsterStats/BPC_MonsterStats.BPC_MonsterStats_C|GetCurrentHealth (Variables|Default|GetBPC_MonsterStats)) 0.0)
        (Utilities|FlowControl|DoOnce false :!label _label_2
          (:Completed
            (Components|Movement|StopMovementImmediately (Variables|Character|GetCharacterMovement))
            (Default|SetStateasHitState _asac_enemy_base)
            (Animation|Montage|PlayMontage (Variables|Character|GetMesh) "/Game/1_Animations/Character/Hit_React/HitReactMonster_UE_Montage.HitReactMonster_UE_Montage" 0.5
              (:then
                (bind _asbp_top_down_character (Utilities|Casting|CastToBP_TopDownCharacter (Game|GetPlayerCharacter 0)))
                (Transformation|SetActorRotation (Math|Rotator|FindLookatRotation (Math|Vector|GetForwardVector (Transformation|GetActorRotation _asbp_top_down_character)) (Transformation|GetActorForwardVector self)))
                (Character|LaunchCharacter (* (Math|Vector|GetForwardVector (Transformation|GetActorRotation _asbp_top_down_character)) 5e+01) false false)
                (goto _label_2 Reset)))))
        (else
          (CallFunction|Death))))
    (:then_2
      (if (<= (/ (Variables|/Game/3_Blueprint/MonsterStats/BPC_MonsterStats.BPC_MonsterStats_C|GetCurrentHealth _bpc_monsterstats) (Variables|/Game/3_Blueprint/MonsterStats/BPC_MonsterStats.BPC_MonsterStats_C|GetMaxHealth _bpc_monsterstats)) 0.5)
        (goto _label)))))

(event EventAttack
  (bind _mesh (Variables|Character|GetMesh))
  (bind _returnvalue (Transformation|GetWorldLocation _mesh))
  (bind _asac_enemy_base (Utilities|Casting|CastToAC_Enemy_base (AI|GetAIController self)))
  (if (== (Utilities|Enum|LiteralenumAI_States "NewEnumerator1") (Class|BlackboardComponent|GetValueasEnum (Variables|/Script/AIModule.AIController|GetBlackboard _asac_enemy_base) (Utilities|Name|MakeLiteralName "States")))
    (Animation|Montage|PlayMontage (Variables|Character|GetMesh) "/Game/Enemies/BasicAnimations/Melee/Montage_Sword_Slash.Montage_Sword_Slash"
      (:OnCompleted
        _)
      (:OnInterrupted
        _))
    (Default|CallAttackFinish)
    (elif (== (Utilities|Enum|LiteralenumAI_States "NewEnumerator5") (Class|BlackboardComponent|GetValueasEnum (Variables|/Script/AIModule.AIController|GetBlackboard _asac_enemy_base) (Utilities|Name|MakeLiteralName "States")))
      (Animation|Montage|PlayMontage (Variables|Character|GetMesh) "/Game/Enemies/BasicAnimations/Rifle/Montage_Rifle_Fire.Montage_Rifle_Fire"
        (:OnCompleted
          _)
        (:OnInterrupted
          _))
      (Default|CallAttackFinish)
      (Game|SpawnActorfromClass "/Game/Enemies/Projectiles/BP_Projectile_0.BP_Projectile_0_C" (Math|Transform|MakeTransform _returnvalue (Math|Rotator|FindLookatRotation _returnvalue (Transformation|GetWorldLocation (Variables|/Script/Engine.Character|GetCapsuleComponent (Game|GetPlayerCharacter 0)))) "1.000000,1.000000,1.000000") "Undefined" "OverrideRootScale" self (Variables|/Game/3_Blueprint/MonsterStats/BPC_MonsterStats.BPC_MonsterStats_C|GetcurrentDamage (Variables|Default|GetBPC_MonsterStats)) 5e+02 0.0 0))))

(fn ConstructionScript
  (|CallParentFunction))