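; Melee enemy Blueprint that performs a sword slash and damages the top-down player character.
; Attack plays the slash montage and signals attack finish when it completes or is interrupted.
; StartSwordTrace and StopSwordTrace control a fast looping timer that sphere-traces between two arrow components, with debug drawing.
; Player hits apply the monster's current damage and trigger OnHit, throttled by a DoOnce that resets after a short delay.
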(event EventBeginPlay
  (|CallParentFunction) ; This node is disabled and will not be called.\nDrag off pins to build functionality.
)

(event Collision|EventActorBeginOverlap
  (params (OtherActor :type Actor%20Object%20Reference))
  (|CallParentFunction OtherActor) ; This node is disabled and will not be called.\nDrag off pins to build functionality.
)

(event EventTick
  (params (DeltaSeconds :type Float%20%28single-precision%29))
  (|CallParentFunction DeltaSeconds) ; This node is disabled and will not be called.\nDrag off pins to build functionality.
)

(event EventAttack
  (Animation|Montage|PlayMontage (Variables|Character|GetMesh) "/Game/Enemies/BasicAnimations/Melee/Montage_Sword_Slash.Montage_Sword_Slash"
    (:OnCompleted
      _)
    (:OnInterrupted
      _))
  (Default|CallAttackFinish))

(event Custom|StopSwordTrace
  (Utilities|Time|ClearandInvalidateTimerbyHandle (Variables|Default|GetSword%20Trace)))

(event Custom|StartSwordTrace
  (params (HitFeedback :type Feedback%20Structure))
  (bind _returnvalue (Utilities|Time|SetTimerbyEvent (delegate Custom|SwordTraceLoop) 0.001 true))
  (Variables|Default|SetSword%20Trace _returnvalue))

(event Custom|SwordTraceLoop
  (bind (_outhit _returnvalue) (Collision|SphereTraceByChannel (Transformation|GetWorldLocation (Variables|Default|GetArrow1)) (Transformation|GetWorldLocation (Variables|Default|GetArrow2)) 15.0 "TraceTypeQuery4" false 0 "ForDuration" true "(R=1.000000,G=0.000000,B=0.000000,A=1.000000)" "(R=0.000000,G=1.000000,B=0.000000,A=1.000000)" 1.0))
  (if _returnvalue
    (Utilities|FlowControl|DoOnce false :!label _label
      (:Completed
        (bind _asbp_top_down_character (Utilities|Casting|CastToBP_TopDownCharacter (.HitActor (Collision|BreakHitResult _outhit))))
        (Default|ChangeHealth (Variables|/Game/Combat_XYH_WeiFu/Blueprints/BP_TopDownCharacter.BP_TopDownCharacter_C|GetBPC_PlayerStats _asbp_top_down_character) (Variables|/Game/3_Blueprint/MonsterStats/BPC_MonsterStats.BPC_MonsterStats_C|GetcurrentDamage (Variables|Default|GetBPC_MonsterStats)) "NewEnumerator1")
        (Default|OnHit (Variables|/Game/Combat_XYH_WeiFu/Blueprints/BP_TopDownCharacter.BP_TopDownCharacter_C|GetBPC_AttackSystem _asbp_top_down_character))
        (Utilities|FlowControl|Delay 0.2)
        (goto _label Reset)))))

(fn ConstructionScript
  (|CallParentFunction))