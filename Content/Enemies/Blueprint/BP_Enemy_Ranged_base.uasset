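; BP_Enemy_Ranged_base is a base ranged enemy that shoots projectiles at the player.
; Attack plays a rifle fire montage, then, whether completed or interrupted, signals attack finish and spawns a projectile from an arrow component, aimed at the player's capsule.
; Damage comes from the monster stats component.
; Override-style functions supply walk speed per movement state, ideal attack and defense ranges, and the stats component.
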(event EventBeginPlay
  (|CallParentFunction) ; This node is disabled and will not be called.\nDrag off pins to build functionality.
)

(event Collision|EventActorBeginOverlap
  (params (OtherActor :type Actor%20Object%20Reference))
  (|CallParentFunction OtherActor) ; This node is disabled and will not be called.\nDrag off pins to build functionality.
)

(event EventTick
  (params (DeltaSeconds :type Float%20%28single-precision%29))
  (|CallParentFunction DeltaSeconds) ; This node is disabled and will not be called.\nDrag off pins to build functionality.
)

(event EventAttack
  (bind _arrow1 (Variables|Default|GetArrow1))
  (bind _returnvalue (Transformation|GetWorldLocation _arrow1))
  ;[1 1 1] Shoot Projectile
  (Animation|Montage|PlayMontage (Variables|Character|GetMesh) "/Game/Enemies/BasicAnimations/Rifle/Montage_Rifle_Fire.Montage_Rifle_Fire"
    (:OnCompleted
      _)
    (:OnInterrupted
      _))
  (Default|CallAttackFinish)
  (Game|SpawnActorfromClass "/Game/Enemies/Projectiles/BP_Projectile_0.BP_Projectile_0_C" (Math|Transform|MakeTransform _returnvalue (Math|Rotator|FindLookatRotation _returnvalue (Transformation|GetWorldLocation (Variables|/Script/Engine.Character|GetCapsuleComponent (Game|GetPlayerCharacter 0)))) "1.000000,1.000000,1.000000") "Undefined" "OverrideRootScale" self (Variables|/Game/3_Blueprint/MonsterStats/BPC_MonsterStats.BPC_MonsterStats_C|GetcurrentDamage (Variables|Default|GetBPC_MonsterStats)) 5e+02 0.0 0))

(fn ConstructionScript
  (|CallParentFunction))

(fn SetMovementSpeed
  (params (movementSpeed :type E_MovementSpeed%20Enum :default "NewEnumerator0"))
  (bind _output_get (Variables|/Script/Engine.CharacterMovementComponent|SetMaxWalkSpeed (Variables|Character|GetCharacterMovement) (Utilities|Select :Index (Utilities|Enum|ByteToEnumE_MovementSpeed movementSpeed) :NewEnumerator0 0.0 :NewEnumerator1 2e+02 :NewEnumerator2 3e+02 :NewEnumerator3 5e+02)))
  (return _output_get))

(fn GetIdealRange
  (return 6e+02 6e+02))

(fn GetMonsterStats
  (return (Variables|Default|GetBPC_MonsterStats)))