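; AI controller for the first enemy boss that runs the pawn's behavior tree and drives it through Blackboard states.
; On BeginPlay it sets a passive state and copies the pawn's attack and defense radii to the Blackboard.
; Sight or damage perception of the player character sets it as attack target and switches to attacking.
; Helper functions expose hit and ranged-attack states, mixing the generic AI_States enum with the boss-specific one.
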(event OnPerceptionUpdated(AIPerception)
  (params (UpdatedActors :type Array%20of%20Actor%20Object%20References))
  (for _array_element UpdatedActors
    (Utilities|FlowControl|Sequence
      (:then_0
        (bind _sensed (CallFunction|CanSenseActor _array_element "NewEnumerator0"))
        (if _sensed
          (bind _asbp_top_down_character (Utilities|Casting|CastToBP_TopDownCharacter _array_element))
          (CallFunction|HandleSensedSight _asbp_top_down_character)))
      (:then_1
        (bind _sensed_2 (CallFunction|CanSenseActor _array_element "NewEnumerator1"))
        (if _sensed_2
          (bind _asbp_top_down_character_2 (Utilities|Casting|CastToBP_TopDownCharacter _array_element))
          (CallFunction|HandleSensedDamage _asbp_top_down_character_2))))))

(event EventBeginPlay
  ;[1 1 1] event called when ai possess, runs before begin play
  (bind _asbp_top_down_character (Utilities|Casting|CastToBP_TopDownCharacter (Game|GetPlayerCharacter 0)))
  (Variables|Default|SetAs%20BP%20Top%20Down%20Character _asbp_top_down_character)
  (CallFunction|SetStatesasPassive)
  (bind (_attackradius _defenseradius) (Class|Damageable|GetIdealRange(Message) (stale EventPossess PossessedPawn)))
  (AI|Components|Blackboard|SetValueasFloat (Variables|Default|GetBlackboard) (Variables|Default|GetAttackRadiusKeyname) _attackradius)
  (AI|Components|Blackboard|SetValueasFloat (Variables|Default|GetBlackboard) (Variables|Default|GetDefendRadiusKeyName) _defenseradius))

(event EventPossess
  (params (PossessedPawn :type Pawn%20Object%20Reference))
  ;[1 1 1] event called when ai possess, runs before begin play
  (bind _asbp_enemy_boss (Utilities|Casting|CastToBP_Enemy_Boss PossessedPawn))
  (bind _behaviortree (Variables|/Game/Enemies/Blueprint/BP_Enemy_base.BP_Enemy_base_C|GetBehaviorTree _asbp_enemy_boss)
    (:then
      (AI|RunBehaviorTree _behaviortree))
    (:else)))

(fn ConstructionScript)

(fn SetStatesasPassive
  (AI|Components|Blackboard|SetValueasEnum (Variables|Default|GetBlackboard) (Variables|Default|GetStateKeyName) (Utilities|Enum|LiteralenumAI_States_Boss "NewEnumerator0")))

(fn SetStatesasAttackingDefault
  (params (attackTarget :type Actor%20Object%20Reference))
  (AI|Components|Blackboard|SetValueasObject (Variables|Default|GetBlackboard) (Variables|Default|GetAttackTargetKeyName) attackTarget)
  (AI|Components|Blackboard|SetValueasEnum (Variables|Default|GetBlackboard) (Variables|Default|GetStateKeyName) (Utilities|Enum|LiteralenumAI_States_Boss "NewEnumerator1"))
  (Variables|Default|SetAttack%20Target attackTarget))

(fn CanSenseActor
  (params (Actor :type Actor%20Object%20Reference) (Sense :type E_AISenses%20Enum :default "NewEnumerator2"))
  (bind _info (Class|AIPerceptionComponent|GetActorsPerception (Variables|Default|GetAIPerception) Actor))
  (for _array_element (.LastSensedStimuli (Utilities|Struct|BreakActorPerceptionBlueprintInfo _info))
    (bind _returnvalue (Class|AIPerceptionSystem|GetSenseClassforStimulus _array_element))
    (if (== _returnvalue (Utilities|Select :Index Sense :NewEnumerator2 0 :NewEnumerator0 "/Script/AIModule.AISense_Sight" :NewEnumerator1 "/Script/AIModule.AISense_Damage"))
      (return (.bSuccessfullySensed (Utilities|Struct|BreakAIStimulus _array_element)) ""))))

(fn HandleSensedSight
  (params (AttackTarget :type Actor%20Object%20Reference))
  (CallFunction|SetStatesasAttackingDefault AttackTarget))

(fn HandleSensedDamage
  (params (actor :type Actor%20Object%20Reference))
  (CallFunction|SetStatesasAttackingDefault actor))

(fn GetCurrentState
  (return (Utilities|Enum|ByteToEnumAI_States (Class|BlackboardComponent|GetValueasEnum (Variables|Default|GetBlackboard) (Variables|Default|GetStateKeyName)))))

(fn SetStateasHitState
  (AI|Components|Blackboard|SetValueasEnum (Variables|Default|GetBlackboard) (Variables|Default|GetStateKeyName) (Utilities|Enum|LiteralenumAI_States "NewEnumerator2")))

(fn SetStateasSwitchRangedAttack
  (params (Attack%20Target :type Actor%20Object%20Reference))
  (AI|Components|Blackboard|SetValueasObject (Variables|Default|GetBlackboard) (Variables|Default|GetAttackTargetKeyName) Attack%20Target)
  (AI|Components|Blackboard|SetValueasEnum (Variables|Default|GetBlackboard) (Variables|Default|GetStateKeyName) (Utilities|Enum|LiteralenumAI_States "NewEnumerator5"))
  (Variables|Default|SetAttack%20Target Attack%20Target))