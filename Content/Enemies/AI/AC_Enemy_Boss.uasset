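; AI controller for the boss enemy, specializing a parent controller's state-switching functions with boss-specific blackboard values.
; Entering the attacking state writes the target and a boss state enum to the blackboard and caches the target in a variable.
; The default attack state handler re-enters attacking with the actor already stored in the blackboard, doing nothing if none is valid.
; The passive state simply defers to the parent.
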(event EventBeginPlay)

(event EventTick
  (params (DeltaSeconds :type Float%20%28single-precision%29)))

(fn ConstructionScript
  (|CallParentFunction))

(fn SetStatesasPassive
  (|CallParentFunction))

(fn SetStatesasAttacking
  (params (attackTarget :type Actor%20Object%20Reference))
  (AI|Components|Blackboard|SetValueasObject (Variables|Default|GetBlackboard) (Variables|Default|GetAttackTargetKeyName) attackTarget)
  (AI|Components|Blackboard|SetValueasEnum (Variables|Default|GetBlackboard) (Variables|Default|GetStateKeyName) (Utilities|Enum|LiteralenumAI_States_Boss "NewEnumerator1"))
  (Variables|Default|SetAttack%20Target attackTarget))

(fn HandleDefaultAttackState
  (bind _asactor (Utilities|Casting|CastToActor (AI|Components|Blackboard|GetValueasObject (Variables|Default|GetBlackboard) (Variables|Default|GetAttackTargetKeyName))))
  (CallFunction|SetStatesasAttacking _asactor))