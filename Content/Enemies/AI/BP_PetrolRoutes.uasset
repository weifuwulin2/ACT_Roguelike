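; BP_PetrolRoutes is an enemy AI patrol route that defines waypoints as the points of a spline.
; GetSplinePointasWorldPosition returns the world location of the spline point at the current PatrolIndex.
; IncreamentPetroRoute steps the index by Direction and flips that direction on reaching the last or first point, producing a back-and-forth patrol instead of a loop.
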(event Custom|IncreamentPetroRoute
  ;[1 1 1] increamenting the current point
  (bind _output_get (Variables|Default|SetPatrolIndex (+ (Variables|Default|GetPatrolIndex) (Variables|Default|GetDirection))))
  (if (== _output_get (- (Spline|GetNumberOfSplinePoints (Variables|Default|GetPetrol%20Route)) 1))
    (Variables|Default|SetDirection -1)
    (elif (== (Variables|Default|GetPatrolIndex) 0)
      (Variables|Default|SetDirection 1))))

(fn ConstructionScript)

(fn GetSplinePointasWorldPosition
  (return (Spline|GetLocationatSplinePoint (Variables|Default|GetPetrol%20Route) (Variables|Default|GetPatrolIndex) "World")))