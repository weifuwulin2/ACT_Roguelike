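; Enemy AI Blueprint for the NianGao_LiShen level that carries a health bar widget component.
; BeginPlay casts the Healthy component's widget to AI_Blood, caches it and initializes its health to full.
; A custom event billboards the bar toward the player camera, though nothing in this graph calls it.
; The attack animation event (播放攻击动作) is an empty stub.
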(event Custom|播放攻击动作)

(event Custom|CusomEvent
  (bind _healthy (Variables|Default|Gethealthy))
  (Transformation|SetWorldRotation _healthy (Math|Rotator|FindLookatRotation (Transformation|GetWorldLocation _healthy) (Camera|GetCameraLocation (Game|GetPlayerCameraManager 0))) false false))

(event EventBeginPlay
  (bind _asai_blood (Utilities|Casting|CastToAI_Blood (UserInterface|GetUserWidgetObject (Variables|Default|Gethealthy))))
  (bind _output_get (Variables|Default|SetAs%20AI%20Blood _asai_blood))
  (Variables|/Game/Level_NianGao_LiShen/Enemy_AI/AI/AI_Blood.AI_Blood_C|Sethealthy _output_get 1e+02))

(fn ConstructionScript)