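; BP_AOE is an actor that, when Trigger is called, rolls a percentage chance (GaiLv) to fire an explosion around player 0's pawn.
; Success draws a debug sphere, runs a Pawn overlap ignoring the instigator with its results unused, and spawns a scaled blast emitter.
; An explosion sound plays at world origin after a short delay.
; The actor destroys itself when the particles finish; a failed roll only prints a message.
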(event Custom|SpawnBlastEffect
  (bind _returnvalue (Effects|SpawnEmitteratLocation (Variables|Default|GetBlast%20Effect) (Transformation|GetActorLocation (Game|Player|GetPlayerPawn 0)) "0, 0, 0" "2.000000,2.000000,2.000000"))
  (EventDispatchers|AssignOnSystemFinished _returnvalue (delegate Custom|SystemFinish)))

(event Custom|PlayBlastSound
  ;[1 1 1] 音效
  (Utilities|FlowControl|Delay 0.3)
  (Audio|PlaySoundatLocation "/Game/2_Assets/StarterContent/Audio/Explosion01.Explosion01" "0, 0, 0" "0, 0, 0" 1.0 1.0 0.0 0 0 0 0))

(event Custom|SpawnAOESphere
  ;[1 1 1] 球体
  (Rendering|Debug|DrawDebugSphere (Transformation|GetActorLocation (Game|Player|GetPlayerPawn 0)) (Variables|Default|GetSphere%20Radius) 12 "(R=1.000000,G=0.061458,B=0.061458,A=1.000000)" 2.0)
  (Collision|SphereOverlapActors (Transformation|GetActorLocation (Game|Player|GetPlayerPawn 0)) (Variables|Default|GetSphere%20Radius) (Utilities|Array|MakeArray "ObjectTypeQuery3") 0 (Utilities|Array|MakeArray (Game|GetInstigator))))

(event Custom|SystemFinish
  (params (PSystem :type Particle%20System%20Component%20Object%20Reference))
  (Actor|DestroyActor)
  (Development|PrintText "销毁"))

(event Custom|Trigger
  ;[1 1 1] 触发
  (if (>= (Variables|Default|GetGaiLv) (Math|Random|RandomIntegerinRange 1 100))
    (CallFunction|SpawnAOESphere)
    (CallFunction|SpawnBlastEffect)
    (CallFunction|PlayBlastSound)
    (else
      (Development|PrintText "没触发"))))

(event Collision|EventActorBeginOverlap
  (params (OtherActor :type Actor%20Object%20Reference)))

(fn ConstructionScript)