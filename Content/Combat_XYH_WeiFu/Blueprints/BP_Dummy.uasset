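; BP_Dummy is a combat dummy character that reacts to hits and can ragdoll after a delay.
; Damage plays a random hit montage, sets rotation from player and dummy forward vectors, and launches it along the player's forward.
; SetEnemyBodyShake drives a physics blend weight by timeline and adds a delayed bone impulse, defaulting to spine_02.
; A non-looping BeginPlay timer applies that weight below the hit bone only once.
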(event Custom|Rogdoll
  ;[1 1 1] Death ragdol
  (Utilities|FlowControl|Delay 2.5)
  (Physics|SetSimulatePhysics (Variables|Character|GetMesh) true))

(event Custom|SetEnemyBodyShake
  (params (hitBoneName :type Name) (hitDirection :type Vector))
  (bind _mesh (Variables|Character|GetMesh))
  ;[1 1 1] 骨骼抖动
  (if (and (!= hitBoneName "None") (!= hitBoneName "pelvis"))
    (Variables|Default|SetHit%20Bone%20Name hitBoneName)
    (else
      (Variables|Default|SetHit%20Bone%20Name "spine_02")))
  (Utilities|FlowControl|Sequence
    (:then_0
      (bind _新建轨道_0 (Timeline|时间轴 PlayFromStart)
        (:Update
          (Variables|Default|SetBlenderWeight _新建轨道_0))
        (:Finished
          (Class|SkeletalMeshComponent|SetAllBodiesPhysicsBlendWeight _mesh 0.0 false)
          (Class|SkeletalMeshComponent|SetAllBodiesSimulatePhysics _mesh false))))
    (:then_1
      (Utilities|FlowControl|Delay 0.06)
      (if (> (Variables|Default|GetBlenderWeight) 0.0)
        (Physics|AddImpulse (Variables|Character|GetMesh) (* hitDirection "10000.000000,10000.000000,10000.000000") (Variables|Default|GetHit%20Bone%20Name) true)))))

(event Custom|自定义事件
  (bind _hit_bone_name (Variables|Default|GetHit%20Bone%20Name))
  ;[1 1 1] 骨骼抖动
  (if (> (Variables|Default|GetBlenderWeight) 0.0)
    (Class|SkeletalMeshComponent|SetAllBodiesBelowSimulatePhysics (Variables|Character|GetMesh) _hit_bone_name true true)
    (Class|SkeletalMeshComponent|SetAllBodiesBelowPhysicsBlendWeight (Variables|Character|GetMesh) _hit_bone_name (Variables|Default|GetBlenderWeight) false true)))

(event Collision|EventActorBeginOverlap
  (params (OtherActor :type Actor%20Object%20Reference)))

(event EventTick
  (params (DeltaSeconds :type Float%20%28single-precision%29)))

(event Game|Damage|EventAnyDamage
  (params (Damage :type Float%20%28single-precision%29) (DamageType :type Damage%20Type%20Object%20Reference) (InstigatedBy :type Controller%20Object%20Reference) (DamageCauser :type Actor%20Object%20Reference))
  (bind _hitanims (Variables|Default|GethitAnims))
  (Animation|PlayAnimMontage (Utilities|Array|Get(acopy) _hitanims (Math|Random|RandomIntegerinRange 0 (- (Utilities|Array|Length _hitanims) 1))) 1.0 "None")
  (bind _asbp_top_down_character (Utilities|Casting|CastToBP_TopDownCharacter (Game|GetPlayerCharacter 0)))
  (Transformation|SetActorRotation (Math|Rotator|FindLookatRotation (Math|Vector|GetForwardVector (Transformation|GetActorRotation _asbp_top_down_character)) (Transformation|GetActorForwardVector self)))
  (Character|LaunchCharacter (* (Math|Vector|GetForwardVector (Transformation|GetActorRotation _asbp_top_down_character)) 7e+02) false false))

(event EventBeginPlay
  ;[1 1 1] 骨骼抖动
  (Utilities|Time|SetTimerbyEvent (delegate Custom|自定义事件) 0.016667))

(fn ConstructionScript)