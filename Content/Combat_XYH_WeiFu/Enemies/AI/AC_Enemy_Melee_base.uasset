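; Base AI controller for melee enemies that runs their behavior tree from a passive state and switches them to attacking on perception.
; Perception updates check each actor for sight, limited to BP_TopDownCharacter, and damage, which accepts any actor.
; A successful sense writes the target and Attacking state to the Blackboard; nothing here reverts it.
; The damage check compares stimuli against AISenseConfig_Damage, a config class rather than a sense class.
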(event OnPerceptionUpdated(AIPerception)
  (params (UpdatedActors :type Array%20of%20Actor%20Object%20References))
  (for _array_element UpdatedActors
    (Utilities|FlowControl|Sequence
      (:then_0
        (bind _sensed (CallFunction|CanSenseActor _array_element "NewEnumerator0"))
        (bind _asbp_top_down_character (Utilities|Casting|CastToBP_TopDownCharacter _array_element))
        (if _sensed
          (CallFunction|HandleSensedSight _asbp_top_down_character)))
      (:then_1
        (bind _sensed_2 (CallFunction|CanSenseActor _array_element "NewEnumerator1"))
        (if _sensed_2
          (CallFunction|HandleSensedDamage _array_element)
          (else
            (Development|PrintString "Hello")))))))

(event EventPossess
  (params (PossessedPawn :type Pawn%20Object%20Reference))
  ;[1 1 1] event called when ai possess, runs before begin play
  (AI|RunBehaviorTree "/Game/Combat_XYH_WeiFu/Enemies/AI/BT_Enemy_Melee_base.BT_Enemy_Melee_base")
  (CallFunction|SetStatesasPassive))

(fn ConstructionScript)

(fn SetStatesasPassive
  (AI|Components|Blackboard|SetValueasEnum (Variables|Default|GetBlackboard) (Variables|Default|GetStateKeyName) (Utilities|Enum|LiteralenumAI_States "NewEnumerator0")))

(fn SetStatesasAttacking
  (params (attackTarget :type Actor%20Object%20Reference))
  (AI|Components|Blackboard|SetValueasObject (Variables|Default|GetBlackboard) (Variables|Default|GetAttackTargetKeyName) attackTarget)
  (AI|Components|Blackboard|SetValueasEnum (Variables|Default|GetBlackboard) (Variables|Default|GetStateKeyName) (Utilities|Enum|LiteralenumAI_States "NewEnumerator1")))

(fn CanSenseActor
  (params (Actor :type Actor%20Object%20Reference) (Sense :type E_AISenses%20Enum :default "NewEnumerator2"))
  (bind _returnvalue (Utilities|Select :Index Sense :NewEnumerator2 0 :NewEnumerator0 "/Script/AIModule.AISense_Sight" :NewEnumerator1 "/Script/AIModule.AISenseConfig_Damage"))
  (bind _info (Class|AIPerceptionComponent|GetActorsPerception (Variables|Default|GetAIPerception) Actor))
  (for _array_element (.LastSensedStimuli (Utilities|Struct|BreakActorPerceptionBlueprintInfo _info))
    (bind _returnvalue_2 (Class|AIPerceptionSystem|GetSenseClassforStimulus _array_element))
    (if (== _returnvalue_2 _returnvalue)
      (Development|PrintString (Utilities|String|Append "Sensed: " (Utilities|GetClassDisplayName _returnvalue)))
      (return (.bSuccessfullySensed (Utilities|Struct|BreakAIStimulus _array_element)) ""))))

(fn HandleSensedSight
  (params (Actor :type Actor%20Object%20Reference))
  (CallFunction|SetStatesasAttacking Actor))

(fn HandleSensedDamage
  (params (actor :type Actor%20Object%20Reference))
  (CallFunction|SetStatesasAttacking actor))

(fn GetCurrentState
  (return (Utilities|Enum|ByteToEnumAI_States (Class|BlackboardComponent|GetValueasEnum (Variables|Default|GetBlackboard) (Variables|Default|GetStateKeyName)))))